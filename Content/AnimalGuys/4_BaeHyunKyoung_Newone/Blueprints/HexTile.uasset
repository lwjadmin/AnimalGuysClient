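; HexTile is a Blueprint for a disappearing floor tile that temporarily gives way after something overlaps its Box trigger.
; The unfiltered overlap event starts a latent Delay chain that turns the HexTile component purple, then hides the actor and switches the component's collision responses to Overlap.
; Two seconds later the tile reappears and blocks again, keeping the purple material.
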(event `self.Box.OnComponentBeginOverlap`
  (params (OverlappedComponent :type "PrimitiveComponent Object Reference") (OtherActor :type "Actor Object Reference") (OtherComp :type "PrimitiveComponent Object Reference") (OtherBodyIndex :type Integer) (bFromSweep :type Boolean) (SweepResult :type "HitResult Structure (by ref)"))
  (`KismetSystemLibrary.Delay` 0.1)
  (`PrimitiveComponent.SetMaterial` (`self.HexTile`) 0 "/Game/GameShowAssetPack/Materials/Ball/Ball_purple_mat_inst.Ball_purple_mat_inst")
  (`KismetSystemLibrary.Delay` 0.2)
  (`PrimitiveComponent.SetCollisionResponseToAllChannels` (`self.HexTile`) "ECR_Overlap")
  (`self.SetActorHiddenInGame` true)
  (`KismetSystemLibrary.Delay` 2.0)
  (`self.SetActorHiddenInGame` false)
  (`PrimitiveComponent.SetCollisionResponseToAllChannels` (`self.HexTile`) "ECR_Block"))

(fn `UserConstructionScript`)