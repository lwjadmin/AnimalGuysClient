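; BP_TCP is a TCP client actor that sends login ID, password and player name strings to a server.
; On BeginPlay it connects to a hardcoded IP and port and stores the connection ID from the connect and disconnect callbacks.
; Three send functions convert their string to bytes and send it on that connection, disconnecting if the send fails.
; Incoming messages are read as strings, but the result is unused.
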(event `self.ReceiveBeginPlay`
  (`self.Connect` "172.16.2.146" 5001 (delegate `DisConnected`) (delegate `Connected`) (delegate `RecvMessage`))
  (`PrimitiveComponent.SetMaterial` (`self.StaticMesh`) 1 null))

(event `DisConnected`
  (params (ConnectionId :type Integer))
  (set `self.Connection Id` ConnectionId))

(event `Connected`
  (params (ConnectionId :type Integer))
  (set `self.Connection Id` ConnectionId))

(event `RecvMessage`
  (params (ConnectionId :type Integer) (Message :type "Array of Byte (by ref)"))
  (`self.Message_ReadString` Message (`KismetArrayLibrary.Array_Length` Message)))

(fn `TCP_SendID`
  (params (Message :type String))
  (bind _connection_id (`self.Connection Id`))
  (bind _returnvalue (`self.SendData` _connection_id (`self.Conv_StringToBytes` Message)))
  (if (not _returnvalue)
    (`self.Disconnect` _connection_id)))

(fn `TCP_SendPlayerName`
  (params (PlayerName :type String))
  (bind _connection_id (`self.Connection Id`))
  (bind _returnvalue (`self.SendData` _connection_id (`self.Conv_StringToBytes` PlayerName)))
  (if (not _returnvalue)
    (`self.Disconnect` _connection_id)))

(fn `TCP_SendPW`
  (params (PW :type String))
  (bind _connection_id (`self.Connection Id`))
  (bind _returnvalue (`self.SendData` _connection_id (`self.Conv_StringToBytes` PW)))
  (if (not _returnvalue)
    (`self.Disconnect` _connection_id)))

(fn `UserConstructionScript`)