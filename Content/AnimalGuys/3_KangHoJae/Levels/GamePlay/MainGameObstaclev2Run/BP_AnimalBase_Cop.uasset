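; Playable animal character base with movement, jump, MP-costed attack and slide, and hat pickup.
; Req/Res events relay actions; attack and slide states apply through OnRep functions, while Tick decays slide speed and drains or regenerates MP in the PlayerState.
; Tick also rebinds PlayerState Kitty/Piggy/Doggy/Bunny change events every frame, which swap mesh and apply currently identical stats.
; Choice input opens a selection widget; PickUp attaches the nearest overlapping hat, replacing any equipped one.
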(event `self.AttackCapsule.OnComponentHit`
  (params (HitComponent :type "PrimitiveComponent Object Reference") (OtherActor :type "Actor Object Reference") (OtherComp :type "PrimitiveComponent Object Reference") (NormalImpulse :type "Vector Structure") (Hit :type "HitResult Structure (by ref)"))
  ;[1 1 1] IsDamaged
  (`self.ReqAttackEvent`))

(event `ReqAttackEvent`
  ;[1 1 1] IsDamaged
  (`self.ResAttackEvent`))

(event `ResAttackEvent`
  (bind _damage (`self.Damage`))
  ;[1 1 1] IsDamaged
  (`KismetSystemLibrary.PrintString` (`KismetStringLibrary.Conv_BoolToString` _damage))
  (if _damage
    (set `self.IsDamaged` true)))

(event `InputAxis|MoveForward` :overrideparent false
  (params (AxisValue :type "Float (single-precision)"))
  ;[1 1 1] CharacterMovement
  (`self.AddMovementInput` (`KismetMathLibrary.GetForwardVector` (`KismetMathLibrary.MakeRotator` 0.0 0.0 (.yaw (`self.GetControlRotation`)))) AxisValue))

(event `InputAction|Attack`
  (params (Key :type "Key Structure"))
  ;[1 1 1] Attack
  (:`Pressed`
    (`self.ReqAttack` true)))

(event `ReqAttack`
  (params (Attack :type Boolean))
  ;[1 1 1] Attack
  (set `self.Attack` Attack)
  (if (`self.CanUseMP`)
    (bind _asbp_animal_guys_player_state (cast `/Game/AnimalGuys/2_JungGuJin/GameMode/BP_AnimalGuys_PlayerState` (`self.PlayerState`)))
    (if (> (`/Game/AnimalGuys/2_JungGuJin/GameMode/BP_AnimalGuys_PlayerState.CurMP` _asbp_animal_guys_player_state) (`KismetMathLibrary.Conv_IntToDouble` (`self.MP_UseSizeOfAttack`)))
      (bind _isnull (`/Game/AnimalGuys/2_JungGuJin/GameMode/BP_AnimalGuys_PlayerState.UseMPAttack` _asbp_animal_guys_player_state (`KismetMathLibrary.Conv_IntToDouble` (`self.MP_UseSizeOfAttack`))))
      (if _isnull
        (set `self.CanUseMP` false)))))

(event `InputAxis|MoveRight` :overrideparent false
  (params (AxisValue :type "Float (single-precision)"))
  ;[1 1 1] CharacterMovement
  (`self.AddMovementInput` (`KismetMathLibrary.GetRightVector` (`KismetMathLibrary.MakeRotator` 0.0 0.0 (.yaw (`self.GetControlRotation`)))) AxisValue))

(event `InputAxis|Turn` :overrideparent false
  (params (AxisValue :type "Float (single-precision)"))
  ;[1 1 1] CharacterMovement
  (`self.AddControllerYawInput` AxisValue))

(event `InputAction|Slide`
  (params (Key :type "Key Structure"))
  ;[1 1 1] Slide
  (:`Pressed`
    (`self.ReqSlide` true))
  (:`Released`
    (`self.ReqSlide` false)))

(event `ReqSlide`
  (params (Slide :type Boolean))
  ;[1 1 1] Slide
  (set `self.Slide` Slide))

(event `self.ReceiveTick`
  (params (DeltaSeconds :type "Float (single-precision)"))
  (`|ExecutionSequence`
    (:`then_0`
      ;[1 1 1] UseMP
      (if (`self.CanSlide`)
        (if (`self.IsSlide`)
          ;;[1 1 1] Decress the Speed In Slide
          (bind _output_get (set `self.DecressSlideSpeed` (- (`self.DecressSlideSpeed`) 3.0)))
          (set `CharacterMovementComponent.MaxWalkSpeed` _output_get (`self.CharacterMovement`))
          (bind _asbp_animal_guys_player_state (cast `/Game/AnimalGuys/2_JungGuJin/GameMode/BP_AnimalGuys_PlayerState` (`self.PlayerState`)))
          (bind _isnull (`/Game/AnimalGuys/2_JungGuJin/GameMode/BP_AnimalGuys_PlayerState.UseMP_Slide` _asbp_animal_guys_player_state (* (`self.MP_UseSizeOfSlide`) (`GameplayStatics.GetWorldDeltaSeconds`))))
          (if _isnull
            (set `self.CanSlide` false)
            (set `CharacterMovementComponent.MaxWalkSpeed` (`self.RunSpeed`) (`self.CharacterMovement`))
            (set `self.IsSlide` false)))))
    (:`then_1`
      (if (not (`self.IsSlide`))
        (bind _asbp_animal_guys_player_state_2 (cast `/Game/AnimalGuys/2_JungGuJin/GameMode/BP_AnimalGuys_PlayerState` (`self.PlayerState`)))
        (bind _ismor20 (`/Game/AnimalGuys/2_JungGuJin/GameMode/BP_AnimalGuys_PlayerState.Get MP_Slide` _asbp_animal_guys_player_state_2 (* (`self.GetMPSpeed`) (`GameplayStatics.GetWorldDeltaSeconds`))))
        (if _ismor20
          (set `self.CanSlide` true))))
    (:`then_2`
      ;[1 1 1] CharacterChange
      (bind _asbp_animal_guys_player_state_3 (cast `/Game/AnimalGuys/2_JungGuJin/GameMode/BP_AnimalGuys_PlayerState` (`self.PlayerState`)))
      (`|ExecutionSequence`
        (:`then_0`
          (add `/Game/AnimalGuys/2_JungGuJin/GameMode/BP_AnimalGuys_PlayerState.ChangeKitty` _asbp_animal_guys_player_state_3 (delegate `Change0_Kitty`)))
        (:`then_1`
          (add `/Game/AnimalGuys/2_JungGuJin/GameMode/BP_AnimalGuys_PlayerState.ChangePiggy` _asbp_animal_guys_player_state_3 (delegate `Change1_Piggy`)))
        (:`then_2`
          (add `/Game/AnimalGuys/2_JungGuJin/GameMode/BP_AnimalGuys_PlayerState.ChangeDoggy` _asbp_animal_guys_player_state_3 (delegate `Change2_Doggy`)))
        (:`then_3`
          (add `/Game/AnimalGuys/2_JungGuJin/GameMode/BP_AnimalGuys_PlayerState.ChangeBunny` _asbp_animal_guys_player_state_3 (delegate `Change3_Bunny`)))))))

(event `InputAxis|LookUp` :overrideparent false
  (params (AxisValue :type "Float (single-precision)"))
  ;[1 1 1] CharacterMovement
  (`self.AddControllerPitchInput` AxisValue))

(event `InputAction|Jump` :overrideparent false
  (params (Key :type "Key Structure"))
  ;[1 1 1] CharacterMovement
  (:`Pressed`
    (`self.Jump`))
  (:`Released`
    (`self.StopJumping`)))

(event `Change0_Kitty`
  ;[1 1 1] CharacterChange
  (`self.Res0`))

(event `Res0`
  ;[1 1 1] CharacterChange
  (`self.Req0`))

(event `Req0`
  ;[1 1 1] CharacterChange
  (`self.ChangeKitty`))

(event `Res1`
  ;[1 1 1] CharacterChange
  (`self.Req1`))

(event `Req1`
  ;[1 1 1] CharacterChange
  (`self.ChangePiggy`))

(event `Change1_Piggy`
  ;[1 1 1] CharacterChange
  (`self.Res1`))

(event `Change2_Doggy`
  ;[1 1 1] CharacterChange
  (`self.Res2`))

(event `Res2`
  ;[1 1 1] CharacterChange
  (`self.Req2`))

(event `Req2`
  ;[1 1 1] CharacterChange
  (`self.ChangeDoggy`))

(event `Res3`
  ;[1 1 1] CharacterChange
  (`self.Req3`))

(event `Req3`
  ;[1 1 1] CharacterChange
  (`self.ChangeBunny`))

(event `Change3_Bunny`
  ;[1 1 1] CharacterChange
  (`self.Res3`))

(event `InputAction|PickUp`
  (params (Key :type "Key Structure"))
  (:`Pressed`
    (`self.ResPickUp`)))

(event `ResPickUp`
  (bind _nesresthat (`self.GetNearestHat`))
  (`/Engine/EditorBlueprintResources/StandardMacros.IsValid` _nesresthat
    (:`Is Valid`
      (`/Engine/EditorBlueprintResources/StandardMacros.IsValid` (`self.EquipedHat`)
        (:`Is Valid`
          (`self.DisableOwnerHat`))
        (:`Is Not Valid`
          _))
      (`self.EnableOwnerHat` _nesresthat)
      (`self.ReqPickUp` _nesresthat))))

(event `ReqPickUp`
  (params (Hat :type "Actor Object Reference"))
  (`/Engine/EditorBlueprintResources/StandardMacros.IsValid` Hat
    (:`Is Valid`
      (`/Engine/EditorBlueprintResources/StandardMacros.IsValid` (`self.EquipedHat`)
        (:`Is Valid`
          (message `/Game/AnimalGuys/2_JungGuJin/Cloth/Hat/BPI_Cloth.DetachHat` (`self.EquipedHat`)))
        (:`Is Not Valid`
          _))
      (`self.AttachHat` Hat))))

(event `InputAction|Choice`
  (params (Key :type "Key Structure"))
  (bind _returnvalue (`GameplayStatics.GetPlayerController` 0))
  (:`Pressed`
    ;[1 1 1] CreateChoiceWidget
    (bind _returnvalue_2 (`|CreateWidget` null))
    (bind _output_get (set `self.ChoiceUI` _returnvalue_2))
    (`UserWidget.AddToViewport` _output_get 0)
    (`WidgetBlueprintLibrary.SetInputMode_GameAndUIEx` _returnvalue null)
    (set `PlayerController.bShowMouseCursor` true _returnvalue)))

(fn `AttachHat`
  (params (EquipedHat :type "Actor Object Reference"))
  (bind _output_get (set `self.EquipedHat` EquipedHat))
  (message `/Game/AnimalGuys/2_JungGuJin/Cloth/Hat/BPI_Cloth.AttachHat` _output_get self))

(fn `ChangeBunny`
  (`SkeletalMeshComponent.SetAnimInstanceClass` (`self.Mesh`) null)
  (`SkinnedMeshComponent.SetSkinnedAssetAndUpdate` (`self.Mesh`) "/Game/Cute_Little_Animals/Bunny/Mesh/SK_Bunny.SK_Bunny" true)
  (`self.CharacterStat` 30 30 40 800.0 600.0 600.0 100.0 3.0 5.0))

(fn `ChangeDoggy`
  (`SkeletalMeshComponent.SetAnimInstanceClass` (`self.Mesh`) null)
  (`SkinnedMeshComponent.SetSkinnedAssetAndUpdate` (`self.Mesh`) "/Game/Cute_Little_Animals/Doggy/Mesh/SK_Doggy.SK_Doggy" true)
  (`self.CharacterStat` 30 30 40 800.0 600.0 600.0 100.0 3.0 5.0))

(fn `ChangeKitty`
  (`SkeletalMeshComponent.SetAnimInstanceClass` (`self.Mesh`) null)
  (`SkinnedMeshComponent.SetSkinnedAssetAndUpdate` (`self.Mesh`) "/Game/Cute_Little_Animals/Kitty/Mesh/SK_Kitty.SK_Kitty" true)
  (`self.CharacterStat` 30 30 40 800.0 600.0 600.0 100.0 3.0 5.0))

(fn `ChangePiggy`
  (`SkeletalMeshComponent.SetAnimInstanceClass` (`self.Mesh`) null)
  (`SkinnedMeshComponent.SetSkinnedAssetAndUpdate` (`self.Mesh`) "/Game/Cute_Little_Animals/Piggy/Mesh/SK_Piggy.SK_Piggy" true)
  (`self.CharacterStat` 30 30 40 800.0 600.0 600.0 100.0 3.0 5.0))

(fn `CharacterStat`
  (params (GetMPSpeed :type Integer) (MP_UseSizeOfSlide :type Integer) (MP_UseSizeOfAttack :type Integer) (SlideSpeed :type "Float (double-precision)") (RunSpeed :type "Float (double-precision)") (`Jump Z Velocity` :type "Float (double-precision)") (MaxMP :type "Float (double-precision)") (AttackCoolTime :type "Float (double-precision)") (DownTimeLength :type "Float (double-precision)"))
  (set `self.MP_UseSizeOfSlide` MP_UseSizeOfSlide)
  (set `self.DefaultSlideSpeed` SlideSpeed)
  (bind _output_get (set `self.RunSpeed` RunSpeed))
  (set `CharacterMovementComponent.MaxWalkSpeed` _output_get (`self.CharacterMovement`))
  (set `CharacterMovementComponent.JumpZVelocity` `Jump Z Velocity` (`self.CharacterMovement`))
  (bind _asbp_animal_guys_player_state (cast `/Game/AnimalGuys/2_JungGuJin/GameMode/BP_AnimalGuys_PlayerState` (`self.PlayerState`)))
  (set `/Game/AnimalGuys/2_JungGuJin/GameMode/BP_AnimalGuys_PlayerState.MaxMP` MaxMP _asbp_animal_guys_player_state)
  (set `self.AttackCoolTime` AttackCoolTime)
  (set `self.MP_UseSizeOfAttack` MP_UseSizeOfAttack)
  (set `self.GetMPSpeed` GetMPSpeed)
  (set `self.DownTimeLength` DownTimeLength))

(fn `DisableOwnerHat`
  (bind _equipedhat (`self.EquipedHat`))
  (`/Engine/EditorBlueprintResources/StandardMacros.IsValid` _equipedhat
    (:`Is Valid`
      (`self.SetOwner` _equipedhat null))))

(fn `EnableOwnerHat`
  (params (EquipHat :type "Actor Object Reference"))
  (`self.SetOwner` (`self.GetController`)))

(fn `GetNearestHat`
  (returns (NesrestHat :type "Actor Object Reference"))
  (locals (NearestActor :type "Actor Object Reference") (NearestDist :type "Float (double-precision)" :default 122222.0))
  (for _array_element (`PrimitiveComponent.GetOverlappingActors` (`self.CapsuleComponent`) "/Game/AnimalGuys/2_JungGuJin/Cloth/Hat/HatParent/BP_Hat.BP_Hat_C")
    (if (`KismetSystemLibrary.DoesImplementInterface` _array_element "/Game/AnimalGuys/2_JungGuJin/Cloth/Hat/BPI_Cloth.BPI_Cloth_C")
      (bind _returnvalue (`KismetMathLibrary.Vector_Distance` (`self.K2_GetActorLocation`) (`self.K2_GetActorLocation` _array_element)))
      (if (> (`local.NearestDist`) _returnvalue)
        (set `local.NearestDist` _returnvalue)
        (set `local.NearestActor` _array_element))))
  (return (`local.NearestActor`)))

(fn `OnRep_Attack`
  (`self.SetAttack` (`self.Attack`)))

(fn `OnRep_Slide`
  (`self.SetSlide` (`self.Slide`)))

(fn `SetAttack`
  (params (Attack :type Boolean))
  (if Attack
    (bind _asbp_animal_guys_player_state (cast `/Game/AnimalGuys/2_JungGuJin/GameMode/BP_AnimalGuys_PlayerState` (`self.PlayerState`)))
    (if (> (`/Game/AnimalGuys/2_JungGuJin/GameMode/BP_AnimalGuys_PlayerState.CurMP` _asbp_animal_guys_player_state) (`KismetMathLibrary.Conv_IntToDouble` (`self.MP_UseSizeOfAttack`)))
      (set `self.IsAttack` true)
      (set `self.CollisionEnable` true)
      (if (`self.CollisionEnable`)
        _))))

(fn `SetSlide`
  (params (Slide :type Boolean))
  (bind _defaultslidespeed (`self.DefaultSlideSpeed`))
  (if Slide
    (if (`self.CanSlide`)
      (set `self.IsSlide` true)
      (set `CharacterMovementComponent.MaxWalkSpeed` _defaultslidespeed (`self.CharacterMovement`))
      (set `self.DecressSlideSpeed` _defaultslidespeed))
    (else
      (set `self.IsSlide` false)
      (set `CharacterMovementComponent.MaxWalkSpeed` (`self.RunSpeed`) (`self.CharacterMovement`)))))

(fn `UserConstructionScript`)