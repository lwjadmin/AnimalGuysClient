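; Game mode for the MainGameObstaclev2Run level that sets up its HUD and tracks joining players.
; BeginPlay creates and shows the run widget and sets game-only input on player 0.
; PostLogin increments the player count and, if the widget exists, sets its GoalinPlayer to half that count.
; The player array logic is unfinished, with unconnected inputs, stray unused nodes and an author note flagging array problems.
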(event `self.ReceiveBeginPlay`
  (bind _returnvalue (`|CreateWidget` "/Game/AnimalGuys/3_KangHoJae/Levels/GamePlay/MainGameObstaclev2Run/BP_MainGameObstaclev2RunWidget.BP_MainGameObstaclev2RunWidget_C"))
  (bind _output_get (set `self.Obstaclev2RunWidget` _returnvalue))
  (`UserWidget.AddToViewport` _output_get 0)
  (`WidgetBlueprintLibrary.SetInputMode_GameOnly` (`GameplayStatics.GetPlayerController` 0)))

(event `self.K2_PostLogin`
  (params (NewPlayer :type "PlayerController Object Reference"))
  (bind _arrayplayer (`self.ArrayPlayer`))
  (bind _obstaclev2runwidget (`self.Obstaclev2RunWidget`))
  (`parent.K2_PostLogin` NewPlayer)
  ;[1 1 1] 배열 문제 많음
  (bind _output_get (set `self.PlayerCount` (+ (`self.PlayerCount`) 1)))
  (`KismetArrayLibrary.Array_Add` _arrayplayer)
  (`KismetArrayLibrary.Array_Set` _arrayplayer _output_get)
  (`/Engine/EditorBlueprintResources/StandardMacros.IsValid` _obstaclev2runwidget
    (:`Is Valid`
      (set `/Game/AnimalGuys/3_KangHoJae/Levels/GamePlay/MainGameObstaclev2Run/BP_MainGameObstaclev2RunWidget.GoalinPlayer` (/ (`self.PlayerCount`) 2) _obstaclev2runwidget))))

(fn `UserConstructionScript`)