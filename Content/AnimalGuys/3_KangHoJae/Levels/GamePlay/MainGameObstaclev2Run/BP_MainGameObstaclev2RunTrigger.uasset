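; Trigger actor for the MainGameObstaclev2Run level that registers overlaps from BP_AnimalBase_Cop characters with the level's game mode.
; When its collision component is overlapped, it confirms the game mode and actor type, increments CurrentCount, then runs an array Set on the game mode's ArrayPlayer.
; The Set has no visible index or item, and an unreachable branch and unused PlayerCount read suggest unfinished logic.
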(event `self.CollisionComponent.OnComponentBeginOverlap`
  (params (OverlappedComponent :type "PrimitiveComponent Object Reference") (OtherActor :type "Actor Object Reference") (OtherComp :type "PrimitiveComponent Object Reference") (OtherBodyIndex :type Integer) (bFromSweep :type Boolean) (SweepResult :type "HitResult Structure (by ref)"))
  (bind _asgm_main_game_obstaclev_2run (cast `/Game/AnimalGuys/3_KangHoJae/Levels/GamePlay/MainGameObstaclev2Run/GM_MainGameObstaclev2Run` (`GameplayStatics.GetGameMode`)))
  (cast `/Game/AnimalGuys/3_KangHoJae/Levels/GamePlay/MainGameObstaclev2Run/BP_AnimalBase_Cop` OtherActor)
  (set `self.CurrentCount` (+ (`self.CurrentCount`) 1))
  (`KismetArrayLibrary.Array_Set` (`/Game/AnimalGuys/3_KangHoJae/Levels/GamePlay/MainGameObstaclev2Run/GM_MainGameObstaclev2Run.ArrayPlayer` _asgm_main_game_obstaclev_2run)))

(fn `UserConstructionScript`)