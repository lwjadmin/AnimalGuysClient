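; BPA_StartChecker is a start-gate trigger actor for the obstacle run that signals the game mode once all players have arrived.
; On the server, its Cube overlap adds each unique Character to an array.
; When the count equals GM_MainGameObstacleRun's CurPlayerCount, it calls CallBreakWall on that game mode.
; Characters are never removed from the array; clients and failed casts only print debug strings.
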(event `self.Cube.OnComponentBeginOverlap`
  (params (OverlappedComponent :type "PrimitiveComponent Object Reference") (OtherActor :type "Actor Object Reference") (OtherComp :type "PrimitiveComponent Object Reference") (OtherBodyIndex :type Integer) (bFromSweep :type Boolean) (SweepResult :type "HitResult Structure (by ref)"))
  (`/Engine/EditorBlueprintResources/ActorMacros.Switch Has Authority`
    (:`Authority`
      (bind _asgm_main_game_obstacle_run (cast `/Game/AnimalGuys/3_KangHoJae/Levels/GamePlay/MainGameObstacleRun/GM_MainGameObstacleRun` (`GameplayStatics.GetGameMode`))
        (:`then`
          (bind _ascharacter (cast `Character` OtherActor)
            (:`then`
              ;[1 1 1] 입장인원 찾아서 같지않으면 추가
              (if (not (>= (`KismetArrayLibrary.Array_Find` (`self.CharacterArray`) _ascharacter) 0))
                (`KismetArrayLibrary.Array_Add` (`self.CharacterArray`) _ascharacter)
                (if (== (`KismetArrayLibrary.Array_Length` (`self.CharacterArray`)) (`/Game/AnimalGuys/3_KangHoJae/Levels/GamePlay/MainGameObstacleRun/GM_MainGameObstacleRun.CurPlayerCount` _asgm_main_game_obstacle_run))
                  (`/Game/AnimalGuys/3_KangHoJae/Levels/GamePlay/MainGameObstacleRun/GM_MainGameObstacleRun.CallBreakWall` _asgm_main_game_obstacle_run))))
            (:`CastFailed`
              (`KismetSystemLibrary.PrintString` "CastFailed2"))))
        (:`CastFailed`
          (`KismetSystemLibrary.PrintString` "CastFailed1"))))
    (:`Remote`
      (`KismetSystemLibrary.PrintString` "Client"))))

(fn `UserConstructionScript`)