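; Trigger area for the reward stage that eliminates characters entering its mesh and ends the match when one player remains.
; Each new overlap is recorded, gets its character stats set and decrements the GameState's left-player count.
; At one left, it collects winners via Find <= 0, which also matches the first eliminated character.
; It passes winners and a never-filled loser array to GameMode, then shows the HUD reward widget.
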(event `self.StaticMesh.OnComponentBeginOverlap`
  (params (OverlappedComponent :type "PrimitiveComponent Object Reference") (OtherActor :type "Actor Object Reference") (OtherComp :type "PrimitiveComponent Object Reference") (OtherBodyIndex :type Integer) (bFromSweep :type Boolean) (SweepResult :type "HitResult Structure (by ref)"))
  (bind _asbp_animal_guys_character (cast `/Game/AnimalGuys/2_JungGuJin/Character/BP_AnimalGuys_Character` OtherActor))
  (if (not (>= (`KismetArrayLibrary.Array_Find` (`self.OverlappedCharacterArray`) _asbp_animal_guys_character) 0))
    (`KismetArrayLibrary.Array_Add` (`self.OverlappedCharacterArray`) _asbp_animal_guys_character)
    (`/Game/AnimalGuys/2_JungGuJin/Character/BP_AnimalGuys_Character.CharacterStat` _asbp_animal_guys_character 30 0 0 0.0 0.0 0.0 100.0 5.0 3.0)
    (bind _asbp_animal_guys_game_state (cast `/Game/AnimalGuys/2_JungGuJin/GameMode/BP_AnimalGuys_GameState` (`GameplayStatics.GetGameState`)))
    (bind _leftplayercount (`/Game/AnimalGuys/2_JungGuJin/GameMode/BP_AnimalGuys_GameState.LeftPlayerCount` _asbp_animal_guys_game_state))
    (`/Game/AnimalGuys/2_JungGuJin/GameMode/BP_AnimalGuys_GameState.SetLeftPlayerCount` _asbp_animal_guys_game_state (- _leftplayercount 1))
    (if (== 1 _leftplayercount)
      (bind _outactors (`GameplayStatics.GetAllActorsOfClass` "/Game/AnimalGuys/2_JungGuJin/Character/BP_AnimalGuys_Character.BP_AnimalGuys_Character_C"))
      (for _array_element _outactors
        (if (<= (`KismetArrayLibrary.Array_Find` (`self.OverlappedCharacterArray`) _array_element) 0)
          (`KismetArrayLibrary.Array_Add` (`self.WinnerCharacterArray`) _array_element)))
      (`self.ReqProcessFinish`))))

(event `ReqProcessFinish`
  (`KismetSystemLibrary.PrintString` "ReqProcessFinish Called" true true (struct :`G` 0.66 :`B` 1.0 :`A` 1.0) 600.0)
  (bind _asbp_animal_guys_game_mode (cast `/Game/AnimalGuys/2_JungGuJin/GameMode/BP_AnimalGuys_GameMode` (`GameplayStatics.GetGameMode`))
    (:`then`
      (`KismetSystemLibrary.PrintString` "GameMode CastSuccess" true true (struct :`G` 0.66 :`B` 1.0 :`A` 1.0) 600.0)
      (`/Game/AnimalGuys/2_JungGuJin/GameMode/BP_AnimalGuys_GameMode.ProcessFinish` _asbp_animal_guys_game_mode (`self.WinnerCharacterArray`) (`self.LoserCharacterArray`))
      (`self.ResProcessFinish`))
    (:`CastFailed`
      (`KismetSystemLibrary.PrintString` "GameMode CastFailed" true true (struct :`G` 0.66 :`B` 1.0 :`A` 1.0) 600.0))))

(event `ResProcessFinish`
  (bind _asbp_animal_guys_hud (cast `/Game/AnimalGuys/2_JungGuJin/GameMode/BP_AnimalGuys_HUD` (`PlayerController.GetHUD` (`GameplayStatics.GetPlayerController` 0))))
  (`/Game/AnimalGuys/2_JungGuJin/GameMode/BP_AnimalGuys_HUD.ShowRewardWidget` _asbp_animal_guys_hud (`self.WinnerCharacterArray`)))

(fn `UserConstructionScript`)