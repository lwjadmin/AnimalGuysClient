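; BPA_FinishArea is a trigger actor that eliminates overlapping AnimalGuys characters and ends the round when one player remains.
; Each character's first overlap records it, sets its stats and decrements the GameState's LeftPlayerCount.
; At one remaining, characters outside the recorded list become winners and the rest losers.
; Both lists go to GameState ProcessFinish, then player 0's HUD shows the reward widget for the winners.
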(event `self.StaticMesh.OnComponentBeginOverlap`
  (params (OverlappedComponent :type "PrimitiveComponent Object Reference") (OtherActor :type "Actor Object Reference") (OtherComp :type "PrimitiveComponent Object Reference") (OtherBodyIndex :type Integer) (bFromSweep :type Boolean) (SweepResult :type "HitResult Structure (by ref)"))
  (bind _asbp_animal_guys_character (cast `/Game/AnimalGuys/2_JungGuJin/Character/BP_AnimalGuys_Character` OtherActor))
  (if (== (`KismetArrayLibrary.Array_Find` (`self.OverlappedCharacterArray`) _asbp_animal_guys_character) -1)
    (`KismetArrayLibrary.Array_Add` (`self.OverlappedCharacterArray`) _asbp_animal_guys_character)
    (`/Game/AnimalGuys/2_JungGuJin/Character/BP_AnimalGuys_Character.CharacterStat` _asbp_animal_guys_character 30 0 0 0.0 0.0 0.0 100.0 5.0 3.0)
    (bind _asbp_animal_guys_game_state (cast `/Game/AnimalGuys/2_JungGuJin/GameMode/BP_AnimalGuys_GameState` (`GameplayStatics.GetGameState`)))
    (bind _leftplayercount (`/Game/AnimalGuys/2_JungGuJin/GameMode/BP_AnimalGuys_GameState.LeftPlayerCount` _asbp_animal_guys_game_state))
    ;[1 1 1] 최후의 1인이 되었을 경우
    (`/Game/AnimalGuys/2_JungGuJin/GameMode/BP_AnimalGuys_GameState.SetLeftPlayerCount` _asbp_animal_guys_game_state (- _leftplayercount 1))
    (if (== 1 _leftplayercount)
      (bind _outactors (`GameplayStatics.GetAllActorsOfClass` "/Game/AnimalGuys/2_JungGuJin/Character/BP_AnimalGuys_Character.BP_AnimalGuys_Character_C"))
      (for _array_element _outactors
        (if (== (`KismetArrayLibrary.Array_Find` (`self.OverlappedCharacterArray`) _array_element) -1)
          (`KismetArrayLibrary.Array_Add` (`self.WinnerCharacterArray`) _array_element)))
      (set `self.LoserCharacterArray` (`self.OverlappedCharacterArray`))
      (bind _asbp_animal_guys_game_state_2 (cast `/Game/AnimalGuys/2_JungGuJin/GameMode/BP_AnimalGuys_GameState` (`GameplayStatics.GetGameState`)))
      (`/Game/AnimalGuys/2_JungGuJin/GameMode/BP_AnimalGuys_GameState.ProcessFinish` _asbp_animal_guys_game_state_2 (`self.WinnerCharacterArray`) (`self.LoserCharacterArray`))
      (bind _asbp_animal_guys_hud (cast `/Game/AnimalGuys/2_JungGuJin/GameMode/BP_AnimalGuys_HUD` (`PlayerController.GetHUD` (`GameplayStatics.GetPlayerController` 0))))
      (`/Game/AnimalGuys/2_JungGuJin/GameMode/BP_AnimalGuys_HUD.ShowRewardWidget` _asbp_animal_guys_hud (`self.WinnerCharacterArray`)))))

(fn `UserConstructionScript`)