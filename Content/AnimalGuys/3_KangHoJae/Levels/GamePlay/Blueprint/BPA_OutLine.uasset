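; BPA_OutLine is a gameplay boundary actor that returns player characters to a PlayerStart when they leave its mesh volume.
; On BeginPlay it caches every PlayerStart in the level.
; When a BP_AnimalGuys_Character ends overlap with the StaticMesh, it is moved to the current start's location.
; An index then advances and wraps to zero, spreading successive respawns round-robin across the starts.
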(event `self.ReceiveBeginPlay`
  (bind _outactors (`GameplayStatics.GetAllActorsOfClass` "/Script/Engine.PlayerStart"))
  (bind _output_get (set `self.PlayerStartArray` _outactors))
  (set `self.PlayerStartLength` (`KismetArrayLibrary.Array_Length` _output_get))
  (set `self.CurPlayerStartIdx` 0))

(event `self.StaticMesh.OnComponentEndOverlap`
  (params (OverlappedComponent :type "PrimitiveComponent Object Reference") (OtherActor :type "Actor Object Reference") (OtherComp :type "PrimitiveComponent Object Reference") (OtherBodyIndex :type Integer))
  (bind _asbp_animal_guys_character (cast `/Game/AnimalGuys/2_JungGuJin/Character/BP_AnimalGuys_Character` OtherActor))
  (`self.K2_SetActorLocation` _asbp_animal_guys_character (`self.K2_GetActorLocation` (`|GetArrayItem` (`self.PlayerStartArray`) (`self.CurPlayerStartIdx`))) false false)
  (bind _result (`/Engine/EditorBlueprintResources/StandardMacros.IncrementInt` (`self.CurPlayerStartIdx`))
    (:`  `
      (if (>= _result (`self.PlayerStartLength`))
        (set `self.CurPlayerStartIdx` 0)))))

(fn `UserConstructionScript`)