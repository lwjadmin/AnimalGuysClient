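; BP_WaitingWall is a waiting wall that holds until every player in the match has touched it.
; On the server, static mesh hits record each distinct AnimalGuys character in CharacterArray.
; When that count equals GamePlayerCount from the game state, it calls CallBreakWaitingWall on the game mode, which handles the break itself.
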(event `self.StaticMesh.OnComponentHit`
  (params (HitComponent :type "PrimitiveComponent Object Reference") (OtherActor :type "Actor Object Reference") (OtherComp :type "PrimitiveComponent Object Reference") (NormalImpulse :type "Vector Structure") (Hit :type "HitResult Structure (by ref)"))
  (`/Engine/EditorBlueprintResources/ActorMacros.Switch Has Authority`
    (:`Authority`
      (bind _asbp_animal_guys_game_state (cast `/Game/AnimalGuys/2_JungGuJin/GameMode/BP_AnimalGuys_GameState` (`GameplayStatics.GetGameState`)))
      (bind _asbp_animal_guys_character (cast `/Game/AnimalGuys/2_JungGuJin/Character/BP_AnimalGuys_Character` OtherActor))
      (if (not (>= (`KismetArrayLibrary.Array_Find` (`self.CharacterArray`) _asbp_animal_guys_character) 0))
        (`KismetArrayLibrary.Array_Add` (`self.CharacterArray`) _asbp_animal_guys_character)
        (if (== (`KismetArrayLibrary.Array_Length` (`self.CharacterArray`)) (`/Game/AnimalGuys/2_JungGuJin/GameMode/BP_AnimalGuys_GameState.GamePlayerCount` _asbp_animal_guys_game_state))
          (bind _asbp_animal_guys_game_mode (cast `/Game/AnimalGuys/2_JungGuJin/GameMode/BP_AnimalGuys_GameMode` (`GameplayStatics.GetGameMode`)))
          (`KismetSystemLibrary.PrintString` "BreakWall Call!!!")
          (`/Game/AnimalGuys/2_JungGuJin/GameMode/BP_AnimalGuys_GameMode.CallBreakWaitingWall` _asbp_animal_guys_game_mode))))))

(fn `UserConstructionScript`)