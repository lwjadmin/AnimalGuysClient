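; BP_GoalTrigger_RedTeam is a goal trigger that awards the red team a point in the AnimalGuys soccer level.
; When a BP_SoccerBall overlaps its collision component, it increments RedTeamScore in the GM_AnimalGuys_MainGameSoccer game mode.
; After a short delay, it finds the BP_MainGameSoccerTargetPoint and calls SpawnBall on it.
; The trigger itself does not remove the scored ball.
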(event `self.CollisionComponent.OnComponentBeginOverlap`
  (params (OverlappedComponent :type "PrimitiveComponent Object Reference") (OtherActor :type "Actor Object Reference") (OtherComp :type "PrimitiveComponent Object Reference") (OtherBodyIndex :type Integer) (bFromSweep :type Boolean) (SweepResult :type "HitResult Structure (by ref)"))
  ;[1 1 1] RedTeam Score
  (bind _asgm_animal_guys_main_game_soccer (cast `/Game/AnimalGuys/3_KangHoJae/Levels/GamePlay/MainGameSoccerLevel/GM_AnimalGuys_MainGameSoccer` (`GameplayStatics.GetGameMode`)))
  (cast `/Game/AnimalGuys/4_BaeHyunKyoung/MainGameSoccer/BP_SoccerBall` OtherActor)
  (bind _score (`/Game/AnimalGuys/3_KangHoJae/Levels/GamePlay/MainGameSoccerLevel/GM_AnimalGuys_MainGameSoccer.Score` _asgm_animal_guys_main_game_soccer))
  (set `/Game/AnimalGuys/3_KangHoJae/Levels/GamePlay/MainGameSoccerLevel/BP_MainGameSoccerScoreWidget.RedTeamScore` (+ (`/Game/AnimalGuys/3_KangHoJae/Levels/GamePlay/MainGameSoccerLevel/BP_MainGameSoccerScoreWidget.RedTeamScore` _score) 1) _score)
  (`KismetSystemLibrary.Delay` 0.7)
  (bind _returnvalue (`GameplayStatics.GetActorOfClass` "/Game/AnimalGuys/3_KangHoJae/Levels/GamePlay/MainGameSoccerLevel/BP_MainGameSoccerTargetPoint.BP_MainGameSoccerTargetPoint_C"))
  (`/Engine/EditorBlueprintResources/StandardMacros.IsValid` _returnvalue
    (:`Is Valid`
      (`/Game/AnimalGuys/3_KangHoJae/Levels/GamePlay/MainGameSoccerLevel/BP_MainGameSoccerTargetPoint.SpawnBall` _returnvalue))))

(fn `UserConstructionScript`)