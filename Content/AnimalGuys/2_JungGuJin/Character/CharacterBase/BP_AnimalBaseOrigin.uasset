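; Base player character for the networked AnimalGuys game, with movement, jump, MP-gated slide and attack, hit damage and hat pickup.
; Slide and attack replicate through OnRep functions, while Tick drains and refills MP in AnimalState.
; Tick also binds AnimalState events that swap animal mesh and stats (Kitty, Piggy, Doggy, Bunny) and master-pose clothing variants.
; Spinner damage ragdolls the character, then a server timer revives it at a PlayerRevivePoint.
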(event `self.CapsuleComponent.OnComponentHit`
  (params (HitComponent :type "PrimitiveComponent Object Reference") (OtherActor :type "Actor Object Reference") (OtherComp :type "PrimitiveComponent Object Reference") (NormalImpulse :type "Vector Structure") (Hit :type "HitResult Structure (by ref)"))
  ;[1 1 1] Damage to OtherCharacter
  (`/Engine/EditorBlueprintResources/ActorMacros.Switch Has Authority`
    (:`Authority`
      (if (`self.IsAttacking?`)
        (`GameplayStatics.ApplyDamage` OtherActor 1.0 (`self.GetController`))))))

(event `self.ReceiveAnyDamage`
  (params (Damage :type "Float (single-precision)") (DamageType :type "DamageType Object Reference") (InstigatedBy :type "Controller Object Reference") (DamageCauser :type "Actor Object Reference"))
  ;[1 1 1] MyPawn has Damaged
  (`|ExecutionSequence`
    (:`then_0`
      ;;[1 1 1] Damaged to OtherCharacter
      (set `self.IsDamaged` true))
    (:`then_1`
      ;;[1 1 1] Damaged to Actor
      (`|ExecutionSequence`
        (:`then_0`
          ;;;[1 1 1] 충돌하는 액터 캐스팅
          (cast `/Game/AnimalGuys/2_JungGuJin/Blueprint/BP_Spinner_GyujinV7` DamageCauser)
          (`self.Do Ragdoll`))))))

(event `ResRevive`
  ;[1 1 1] MyPawn has Damaged
  ;;[1 1 1] Damaged to Actor
  (`self.DoRevive`))

(event `self.ReceiveBeginPlay`
  ;[1 1 1] SetStartCharacter
  (set `self.IsInLobby?` false)
  (`self.ChangeKitty`))

(event `InputAxis|MoveForward` :overrideparent false
  (params (AxisValue :type "Float (single-precision)"))
  ;[1 1 1] CharacterMovement
  (`self.AddMovementInput` (`KismetMathLibrary.GetForwardVector` (`KismetMathLibrary.MakeRotator` 0.0 0.0 (.yaw (`self.GetControlRotation`)))) AxisValue))

(event `ReqAttack`
  (params (Attack :type Boolean))
  ;[1 1 1] Attack
  (set `self.Attack` Attack)
  (if (`self.CanUseMP`)
    ;;[1 1 1] Use Stamina
    (if (not (`self.IsInLobby?`))
      (bind _asanimal_state (cast `/Game/AnimalGuys/2_JungGuJin/GameMode/AnimalState` (`self.PlayerState`)))
      (if (> (`/Game/AnimalGuys/2_JungGuJin/GameMode/AnimalState.CurMP` _asanimal_state) (`KismetMathLibrary.Conv_IntToDouble` (`self.MP_UseSizeOfAttack`)))
        (bind _isnull (`/Game/AnimalGuys/2_JungGuJin/GameMode/AnimalState.UseMPAttack` _asanimal_state (`KismetMathLibrary.Conv_IntToDouble` (`self.MP_UseSizeOfAttack`))))
        (if _isnull
          (set `self.CanUseMP` false))))))

(event `InputAction|Attack`
  (params (Key :type "Key Structure"))
  ;[1 1 1] Attack
  (:`Pressed`
    ;;[1 1 1] IsJumping?
    (if (not (`self.IsJumping?`))
      (`self.ReqAttack` true))))

(event `InputAxis|MoveRight` :overrideparent false
  (params (AxisValue :type "Float (single-precision)"))
  ;[1 1 1] CharacterMovement
  (`self.AddMovementInput` (`KismetMathLibrary.GetRightVector` (`KismetMathLibrary.MakeRotator` 0.0 0.0 (.yaw (`self.GetControlRotation`)))) AxisValue))

(event `InputAxis|Turn` :overrideparent false
  (params (AxisValue :type "Float (single-precision)"))
  ;[1 1 1] CharacterMovement
  (`self.AddControllerYawInput` AxisValue))

(event `InputAction|Slide`
  (params (Key :type "Key Structure"))
  ;[1 1 1] Slide
  (:`Pressed`
    ;;[1 1 1] IsJumping?
    (if (not (`self.IsJumping?`))
      (`self.ReqSlide` true)))
  (:`Released`
    (`self.ReqSlide` false)))

(event `self.ReceiveTick`
  (params (DeltaSeconds :type "Float (single-precision)"))
  (`|ExecutionSequence`
    (:`then_0`
      (`|ExecutionSequence`
        (:`then_0`
          ;[1 1 1] UseMP
          (if (`self.CanSlide`)
            (if (`self.IsSlide`)
              ;;[1 1 1] Decress the Speed In Slide
              (bind _output_get (set `self.DecressSlideSpeed` (- (`self.DecressSlideSpeed`) 3.0)))
              (set `CharacterMovementComponent.MaxWalkSpeed` _output_get (`self.CharacterMovement`))
              (bind _asanimal_state (cast `/Game/AnimalGuys/2_JungGuJin/GameMode/AnimalState` (`self.PlayerState`)))
              (bind _isnull (`/Game/AnimalGuys/2_JungGuJin/GameMode/AnimalState.UseMP_Slide` _asanimal_state (* (`self.MP_UseSizeOfSlide`) (`GameplayStatics.GetWorldDeltaSeconds`))))
              (if _isnull
                (set `self.CanSlide` false)
                (set `CharacterMovementComponent.MaxWalkSpeed` (`self.RunSpeed`) (`self.CharacterMovement`))
                (set `self.IsSlide` false)))))
        (:`then_1`
          (if (not (`self.IsSlide`))
            (bind _asanimal_state_2 (cast `/Game/AnimalGuys/2_JungGuJin/GameMode/AnimalState` (`self.PlayerState`)))
            (bind _ismor20 (`/Game/AnimalGuys/2_JungGuJin/GameMode/AnimalState.Get MP_Slide` _asanimal_state_2 (* (`self.GetMPSpeed`) (`GameplayStatics.GetWorldDeltaSeconds`))))
            (if _ismor20
              (set `self.CanSlide` true))))))
    (:`then_1`
      ;[1 1 1] CharacterChange
      (bind _asanimal_state_3 (cast `/Game/AnimalGuys/2_JungGuJin/GameMode/AnimalState` (`self.PlayerState`)))
      (`|ExecutionSequence`
        (:`then_0`
          (add `/Game/AnimalGuys/2_JungGuJin/GameMode/AnimalState.ChangeKitty` _asanimal_state_3 (delegate `Change0_Kitty`)))
        (:`then_1`
          (add `/Game/AnimalGuys/2_JungGuJin/GameMode/AnimalState.ChangePiggy` _asanimal_state_3 (delegate `Change1_Piggy`)))
        (:`then_2`
          (add `/Game/AnimalGuys/2_JungGuJin/GameMode/AnimalState.ChangeDoggy` _asanimal_state_3 (delegate `Change2_Doggy`)))
        (:`then_3`
          (add `/Game/AnimalGuys/2_JungGuJin/GameMode/AnimalState.ChangeBunny` _asanimal_state_3 (delegate `Change3_Bunny`)))))
    (:`then_2`
      ;[1 1 1] ClothColorChange
      (bind _asanimal_state_4 (cast `/Game/AnimalGuys/2_JungGuJin/GameMode/AnimalState` (`self.PlayerState`)))
      (`|ExecutionSequence`
        (:`then_0`
          (add `/Game/AnimalGuys/2_JungGuJin/GameMode/AnimalState.ChangeBared` _asanimal_state_4 (delegate `ChangeBared`)))
        (:`then_1`
          (add `/Game/AnimalGuys/2_JungGuJin/GameMode/AnimalState.ChaneA` _asanimal_state_4 (delegate `ChangeA`)))
        (:`then_2`
          (add `/Game/AnimalGuys/2_JungGuJin/GameMode/AnimalState.ChangeB` _asanimal_state_4 (delegate `ChangeB`)))
        (:`then_3`
          (add `/Game/AnimalGuys/2_JungGuJin/GameMode/AnimalState.ChangeC` _asanimal_state_4 (delegate `ChangeC`)))))))

(event `InputAxis|LookUp` :overrideparent false
  (params (AxisValue :type "Float (single-precision)"))
  ;[1 1 1] CharacterMovement
  (`self.AddControllerPitchInput` AxisValue))

(event `InputAction|Jump` :overrideparent false
  (params (Key :type "Key Structure"))
  ;[1 1 1] CharacterMovement
  (:`Pressed`
    (`self.Jump`))
  (:`Released`
    (`self.StopJumping`)))

(event `ReqSlide`
  (params (Slide :type Boolean))
  ;[1 1 1] Slide
  (set `self.Slide` Slide))

(event `Change0_Kitty`
  ;[1 1 1] CharacterChange
  (`self.Res0`))

(event `Res0`
  ;[1 1 1] CharacterChange
  (`self.Req0`))

(event `Req0`
  ;[1 1 1] CharacterChange
  (`self.ChangeKitty`))

(event `Res1`
  ;[1 1 1] CharacterChange
  (`self.Req1`))

(event `Req1`
  ;[1 1 1] CharacterChange
  (`self.ChangePiggy`))

(event `Change1_Piggy`
  ;[1 1 1] CharacterChange
  (`self.Res1`))

(event `Res2`
  ;[1 1 1] CharacterChange
  (`self.Req2`))

(event `Req2`
  ;[1 1 1] CharacterChange
  (`self.ChangeDoggy`))

(event `Change2_Doggy`
  ;[1 1 1] CharacterChange
  (`self.Res2`))

(event `Res3`
  ;[1 1 1] CharacterChange
  (`self.Req3`))

(event `Req3`
  ;[1 1 1] CharacterChange
  (`self.ChangeBunny`))

(event `Change3_Bunny`
  ;[1 1 1] CharacterChange
  (`self.Res3`))

(event `ResBared`
  ;[1 1 1] ClothColorChange
  (`self.ReqBared`))

(event `ReqBared`
  ;[1 1 1] ClothColorChange
  (`self.Bared`))

(event `ChangeBared`
  ;[1 1 1] ClothColorChange
  (`self.ResBared`))

(event `ResA`
  ;[1 1 1] ClothColorChange
  (`self.ReqA`))

(event `ReqA`
  ;[1 1 1] ClothColorChange
  (`self.A`))

(event `ChangeA`
  ;[1 1 1] ClothColorChange
  (`self.ResA`))

(event `ResB`
  ;[1 1 1] ClothColorChange
  (`self.ReqB`))

(event `ReqB`
  ;[1 1 1] ClothColorChange
  (`self.B`))

(event `ChangeB`
  ;[1 1 1] ClothColorChange
  (`self.ResB`))

(event `ResC`
  ;[1 1 1] ClothColorChange
  (`self.ReqC`))

(event `ReqC`
  ;[1 1 1] ClothColorChange
  (`self.C`))

(event `ChangeC`
  ;[1 1 1] ClothColorChange
  (`self.ResC`))

(event `InputAction|PickUp`
  (params (Key :type "Key Structure"))
  (:`Pressed`
    (`self.ResPickUp`)))

(event `ResPickUp`
  (bind _nesresthat (`self.GetNearestHat`))
  (`/Engine/EditorBlueprintResources/StandardMacros.IsValid` _nesresthat
    (:`Is Valid`
      (`/Engine/EditorBlueprintResources/StandardMacros.IsValid` (`self.EquipedHat`)
        (:`Is Valid`
          (`self.DisableOwnerHat`))
        (:`Is Not Valid`
          _))
      (`self.EnableOwnerHat` _nesresthat)
      (`self.ReqPickUp` _nesresthat))))

(event `ReqPickUp`
  (params (Hat :type "Actor Object Reference"))
  (`/Engine/EditorBlueprintResources/StandardMacros.IsValid` Hat
    (:`Is Valid`
      (`/Engine/EditorBlueprintResources/StandardMacros.IsValid` (`self.EquipedHat`)
        (:`Is Valid`
          (message `/Game/AnimalGuys/2_JungGuJin/Cloth/Hat/BPI_Cloth.DetachHat` (`self.EquipedHat`)))
        (:`Is Not Valid`
          _))
      (`self.AttachHat` Hat))))

(event `InputAction|Choice`
  (params (Key :type "Key Structure"))
  (bind _returnvalue (`GameplayStatics.GetPlayerController` 0))
  (:`Pressed`
    ;[1 1 1] CreateChoiceWidget
    (bind _returnvalue_2 (`|CreateWidget` "/Game/AnimalGuys/2_JungGuJin/Widget/CharacterChoiceWidget.CharacterChoiceWidget_C"))
    (bind _output_get (set `self.ChoiceUI` _returnvalue_2))
    (`UserWidget.AddToViewport` _output_get 0)
    (`WidgetBlueprintLibrary.SetInputMode_GameAndUIEx` _returnvalue null)
    (set `PlayerController.bShowMouseCursor` true _returnvalue)))

(fn `A`
  (bind _skeletalmesh (`self.SkeletalMesh`))
  (bind _skeletalmesh_2 (`self.SkeletalMesh`))
  (bind _skeletalmesh_3 (`self.SkeletalMesh`))
  (bind _skeletalmesh_4 (`self.SkeletalMesh`))
  (bind _skeletalmesh_5 (`self.SkeletalMesh`))
  (`SceneComponent.SetVisibility` _skeletalmesh_3 true false)
  (cast `/Game/AnimalGuys/2_JungGuJin/GameMode/AnimalState` (`self.PlayerState`))
  (switch `int` (`self.AnimalType`)
    (:`0`
      (`PrimitiveComponent.SetMaterial` _skeletalmesh_3 0 "/Game/AnimalGuys/2_JungGuJin/Character/0_Kitty/Material/MI_Kitty_A.MI_Kitty_A")
      (`SkeletalMeshComponent.SetAnimInstanceClass` _skeletalmesh_4 "/Game/AnimalGuys/2_JungGuJin/Character/0_Kitty/Animation/ABP_AnimalKitty.ABP_AnimalKitty_C")
      (`SkinnedMeshComponent.SetSkinnedAssetAndUpdate` _skeletalmesh_4 "/Game/AnimalGuys/2_JungGuJin/Character/0_Kitty/Mesh/SK_Kitty_MyClothes.SK_Kitty_MyClothes" true)
      (`SkinnedMeshComponent.SetLeaderPoseComponent` _skeletalmesh_4 (`self.Mesh`) false))
    (:`1`
      (`PrimitiveComponent.SetMaterial` _skeletalmesh_3 0 "/Game/AnimalGuys/2_JungGuJin/Character/1_Piggy/Material/MI_Piggy_A.MI_Piggy_A")
      (`SkeletalMeshComponent.SetAnimInstanceClass` _skeletalmesh "/Game/AnimalGuys/2_JungGuJin/Character/1_Piggy/Animation/ABP_AnimalPiggy.ABP_AnimalPiggy_C")
      (`SkinnedMeshComponent.SetSkinnedAssetAndUpdate` _skeletalmesh "/Game/Cute_Little_Animals/Piggy/Mesh/SK_Piggy_Clothes.SK_Piggy_Clothes" true)
      (`SkinnedMeshComponent.SetLeaderPoseComponent` _skeletalmesh (`self.Mesh`) false))
    (:`2`
      (`PrimitiveComponent.SetMaterial` _skeletalmesh_3 0 "/Game/AnimalGuys/2_JungGuJin/Character/3_Doggy/Material/MI_Doggy_A.MI_Doggy_A")
      (`SkeletalMeshComponent.SetAnimInstanceClass` _skeletalmesh_2 "/Game/AnimalGuys/2_JungGuJin/Character/3_Doggy/Animation/ABP_AnimDoggy.ABP_AnimDoggy_C")
      (`SkinnedMeshComponent.SetSkinnedAssetAndUpdate` _skeletalmesh_2 "/Game/Cute_Little_Animals/Doggy/Mesh/SK_Doggy_clothes.SK_Doggy_clothes" true)
      (`SkinnedMeshComponent.SetLeaderPoseComponent` _skeletalmesh_2 (`self.Mesh`) false))
    (:`3`
      (`PrimitiveComponent.SetMaterial` _skeletalmesh_3 0 "/Game/AnimalGuys/2_JungGuJin/Character/4_Bunny/Material/MI_Bunny_A.MI_Bunny_A")
      (`SkeletalMeshComponent.SetAnimInstanceClass` _skeletalmesh_5 "/Game/AnimalGuys/2_JungGuJin/Character/4_Bunny/Animation/ABP_AnimBunny.ABP_AnimBunny_C")
      (`SkinnedMeshComponent.SetSkinnedAssetAndUpdate` _skeletalmesh_5 "/Game/Cute_Little_Animals/Bunny/Mesh/SK_Bunny_Clothes.SK_Bunny_Clothes" true)
      (`SkinnedMeshComponent.SetLeaderPoseComponent` _skeletalmesh_5 (`self.Mesh`) false))))

(fn `AttachHat`
  (params (EquipedHat :type "Actor Object Reference"))
  (bind _output_get (set `self.EquipedHat` EquipedHat))
  (message `/Game/AnimalGuys/2_JungGuJin/Cloth/Hat/BPI_Cloth.AttachHat` _output_get self))

(fn `B`
  (bind _skeletalmesh (`self.SkeletalMesh`))
  (bind _skeletalmesh_2 (`self.SkeletalMesh`))
  (bind _skeletalmesh_3 (`self.SkeletalMesh`))
  (bind _skeletalmesh_4 (`self.SkeletalMesh`))
  (bind _skeletalmesh_5 (`self.SkeletalMesh`))
  (`SceneComponent.SetVisibility` _skeletalmesh_3 true false)
  (cast `/Game/AnimalGuys/2_JungGuJin/GameMode/AnimalState` (`self.PlayerState`))
  (switch `int` (`self.AnimalType`)
    (:`0`
      (`PrimitiveComponent.SetMaterial` _skeletalmesh_3 0 "/Game/AnimalGuys/2_JungGuJin/Character/0_Kitty/Material/MI_Kitty_B.MI_Kitty_B")
      (`SkeletalMeshComponent.SetAnimInstanceClass` _skeletalmesh_4 "/Game/AnimalGuys/2_JungGuJin/Character/0_Kitty/Animation/ABP_AnimalKitty.ABP_AnimalKitty_C")
      (`SkinnedMeshComponent.SetSkinnedAssetAndUpdate` _skeletalmesh_4 "/Game/AnimalGuys/2_JungGuJin/Character/0_Kitty/Mesh/SK_Kitty_MyClothes.SK_Kitty_MyClothes" true)
      (`SkinnedMeshComponent.SetLeaderPoseComponent` _skeletalmesh_4 (`self.Mesh`) false))
    (:`1`
      (`PrimitiveComponent.SetMaterial` _skeletalmesh_3 0 "/Game/AnimalGuys/2_JungGuJin/Character/1_Piggy/Material/MI_Piggy_B.MI_Piggy_B")
      (`SkeletalMeshComponent.SetAnimInstanceClass` _skeletalmesh "/Game/AnimalGuys/2_JungGuJin/Character/1_Piggy/Animation/ABP_AnimalPiggy.ABP_AnimalPiggy_C")
      (`SkinnedMeshComponent.SetSkinnedAssetAndUpdate` _skeletalmesh "/Game/Cute_Little_Animals/Piggy/Mesh/SK_Piggy_Clothes.SK_Piggy_Clothes" true)
      (`SkinnedMeshComponent.SetLeaderPoseComponent` _skeletalmesh (`self.Mesh`) false))
    (:`2`
      (`PrimitiveComponent.SetMaterial` _skeletalmesh_3 0 "/Game/AnimalGuys/2_JungGuJin/Character/3_Doggy/Material/MI_Doggy_B.MI_Doggy_B")
      (`SkeletalMeshComponent.SetAnimInstanceClass` _skeletalmesh_2 "/Game/AnimalGuys/2_JungGuJin/Character/3_Doggy/Animation/ABP_AnimDoggy.ABP_AnimDoggy_C")
      (`SkinnedMeshComponent.SetSkinnedAssetAndUpdate` _skeletalmesh_2 "/Game/Cute_Little_Animals/Doggy/Mesh/SK_Doggy_clothes.SK_Doggy_clothes" true)
      (`SkinnedMeshComponent.SetLeaderPoseComponent` _skeletalmesh_2 (`self.Mesh`) false))
    (:`3`
      (`PrimitiveComponent.SetMaterial` _skeletalmesh_3 0 "/Game/AnimalGuys/2_JungGuJin/Character/4_Bunny/Material/MI_Bunny_B.MI_Bunny_B")
      (`SkeletalMeshComponent.SetAnimInstanceClass` _skeletalmesh_5 "/Game/AnimalGuys/2_JungGuJin/Character/4_Bunny/Animation/ABP_AnimBunny.ABP_AnimBunny_C")
      (`SkinnedMeshComponent.SetSkinnedAssetAndUpdate` _skeletalmesh_5 "/Game/Cute_Little_Animals/Bunny/Mesh/SK_Bunny_Clothes.SK_Bunny_Clothes" true)
      (`SkinnedMeshComponent.SetLeaderPoseComponent` _skeletalmesh_5 (`self.Mesh`) false))))

(fn `Bared`
  (cast `/Game/AnimalGuys/2_JungGuJin/GameMode/AnimalState` (`self.PlayerState`))
  (switch `int` (`self.AnimalType`)
    (:`0`
      _)
    (:`1`
      _)
    (:`2`
      _)
    (:`3`
      _))
  (`SceneComponent.SetVisibility` (`self.SkeletalMesh`) false false))

(fn `C`
  (bind _skeletalmesh (`self.SkeletalMesh`))
  (bind _skeletalmesh_2 (`self.SkeletalMesh`))
  (bind _skeletalmesh_3 (`self.SkeletalMesh`))
  (bind _skeletalmesh_4 (`self.SkeletalMesh`))
  (bind _skeletalmesh_5 (`self.SkeletalMesh`))
  (`SceneComponent.SetVisibility` _skeletalmesh_3 true false)
  (cast `/Game/AnimalGuys/2_JungGuJin/GameMode/AnimalState` (`self.PlayerState`))
  (switch `int` (`self.AnimalType`)
    (:`0`
      (`PrimitiveComponent.SetMaterial` _skeletalmesh_3 0 "/Game/AnimalGuys/2_JungGuJin/Character/0_Kitty/Material/MI_Kitty_C.MI_Kitty_C")
      (`SkeletalMeshComponent.SetAnimInstanceClass` _skeletalmesh_4 "/Game/AnimalGuys/2_JungGuJin/Character/0_Kitty/Animation/ABP_AnimalKitty.ABP_AnimalKitty_C")
      (`SkinnedMeshComponent.SetSkinnedAssetAndUpdate` _skeletalmesh_4 "/Game/AnimalGuys/2_JungGuJin/Character/0_Kitty/Mesh/SK_Kitty_MyClothes.SK_Kitty_MyClothes" true)
      (`SkinnedMeshComponent.SetLeaderPoseComponent` _skeletalmesh_4 (`self.Mesh`) false))
    (:`1`
      (`PrimitiveComponent.SetMaterial` _skeletalmesh_3 0 "/Game/AnimalGuys/2_JungGuJin/Character/1_Piggy/Material/MI_Piggy_C.MI_Piggy_C")
      (`SkeletalMeshComponent.SetAnimInstanceClass` _skeletalmesh "/Game/AnimalGuys/2_JungGuJin/Character/1_Piggy/Animation/ABP_AnimalPiggy.ABP_AnimalPiggy_C")
      (`SkinnedMeshComponent.SetSkinnedAssetAndUpdate` _skeletalmesh "/Game/Cute_Little_Animals/Piggy/Mesh/SK_Piggy_Clothes.SK_Piggy_Clothes" true)
      (`SkinnedMeshComponent.SetLeaderPoseComponent` _skeletalmesh (`self.Mesh`) false))
    (:`2`
      (`PrimitiveComponent.SetMaterial` _skeletalmesh_3 0 "/Game/AnimalGuys/2_JungGuJin/Character/3_Doggy/Material/MI_Doggy_C.MI_Doggy_C")
      (`SkeletalMeshComponent.SetAnimInstanceClass` _skeletalmesh_2 "/Game/AnimalGuys/2_JungGuJin/Character/3_Doggy/Animation/ABP_AnimDoggy.ABP_AnimDoggy_C")
      (`SkinnedMeshComponent.SetSkinnedAssetAndUpdate` _skeletalmesh_2 "/Game/Cute_Little_Animals/Doggy/Mesh/SK_Doggy_clothes.SK_Doggy_clothes" true)
      (`SkinnedMeshComponent.SetLeaderPoseComponent` _skeletalmesh_2 (`self.Mesh`) false))
    (:`3`
      (`PrimitiveComponent.SetMaterial` _skeletalmesh_3 0 "/Game/AnimalGuys/2_JungGuJin/Character/4_Bunny/Material/MI_Bunny_C.MI_Bunny_C")
      (`SkeletalMeshComponent.SetAnimInstanceClass` _skeletalmesh_5 "/Game/AnimalGuys/2_JungGuJin/Character/4_Bunny/Animation/ABP_AnimBunny.ABP_AnimBunny_C")
      (`SkinnedMeshComponent.SetSkinnedAssetAndUpdate` _skeletalmesh_5 "/Game/Cute_Little_Animals/Bunny/Mesh/SK_Bunny_Clothes.SK_Bunny_Clothes" true)
      (`SkinnedMeshComponent.SetLeaderPoseComponent` _skeletalmesh_5 (`self.Mesh`) false))))

(fn `ChangeBunny`
  (`SceneComponent.SetVisibility` (`self.SkeletalMesh`) false false)
  (`SkeletalMeshComponent.SetAnimInstanceClass` (`self.Mesh`) "/Game/AnimalGuys/2_JungGuJin/Character/4_Bunny/Animation/ABP_AnimBunny.ABP_AnimBunny_C")
  (`SkinnedMeshComponent.SetSkinnedAssetAndUpdate` (`self.Mesh`) "/Game/Cute_Little_Animals/Bunny/Mesh/SK_Bunny.SK_Bunny" true)
  (`self.CharacterStat` 30 30 40 800.0 600.0 600.0 100.0 3.0 2.0)
  (set `self.AnimalType` 3))

(fn `ChangeDoggy`
  (`SceneComponent.SetVisibility` (`self.SkeletalMesh`) false false)
  (`SkeletalMeshComponent.SetAnimInstanceClass` (`self.Mesh`) "/Game/AnimalGuys/2_JungGuJin/Character/3_Doggy/Animation/ABP_AnimDoggy.ABP_AnimDoggy_C")
  (`SkinnedMeshComponent.SetSkinnedAssetAndUpdate` (`self.Mesh`) "/Game/Cute_Little_Animals/Doggy/Mesh/SK_Doggy.SK_Doggy" true)
  (`self.CharacterStat` 30 30 40 800.0 600.0 600.0 100.0 3.0 2.0)
  (set `self.AnimalType` 2))

(fn `ChangeKitty`
  (`SceneComponent.SetVisibility` (`self.SkeletalMesh`) false false)
  (`SkeletalMeshComponent.SetAnimInstanceClass` (`self.Mesh`) "/Game/AnimalGuys/2_JungGuJin/Character/0_Kitty/Animation/ABP_AnimalKitty.ABP_AnimalKitty_C")
  (`SkinnedMeshComponent.SetSkinnedAssetAndUpdate` (`self.Mesh`) "/Game/Cute_Little_Animals/Kitty/Mesh/SK_Kitty.SK_Kitty" true)
  (`self.CharacterStat` 30 30 40 800.0 600.0 600.0 100.0 3.0 2.0)
  (set `self.AnimalType` 0))

(fn `ChangePiggy`
  (`SceneComponent.SetVisibility` (`self.SkeletalMesh`) false false)
  (`SkeletalMeshComponent.SetAnimInstanceClass` (`self.Mesh`) "/Game/AnimalGuys/2_JungGuJin/Character/1_Piggy/Animation/ABP_AnimalPiggy.ABP_AnimalPiggy_C")
  (`SkinnedMeshComponent.SetSkinnedAssetAndUpdate` (`self.Mesh`) "/Game/Cute_Little_Animals/Piggy/Mesh/SK_Piggy.SK_Piggy" true)
  (`self.CharacterStat` 30 30 40 800.0 600.0 600.0 100.0 3.0 2.0)
  (set `self.AnimalType` 1))

(fn `CharacterStat`
  (params (GetMPSpeed :type Integer) (MP_UseSizeOfSlide :type Integer) (MP_UseSizeOfAttack :type Integer) (SlideSpeed :type "Float (double-precision)") (RunSpeed :type "Float (double-precision)") (`Jump Z Velocity` :type "Float (double-precision)") (MaxMP :type "Float (double-precision)") (AttackCoolTime :type "Float (double-precision)") (DownTimeLength :type "Float (double-precision)"))
  (set `self.MP_UseSizeOfSlide` MP_UseSizeOfSlide)
  (set `self.DefaultSlideSpeed` SlideSpeed)
  (bind _output_get (set `self.RunSpeed` RunSpeed))
  (set `CharacterMovementComponent.MaxWalkSpeed` _output_get (`self.CharacterMovement`))
  (set `CharacterMovementComponent.JumpZVelocity` `Jump Z Velocity` (`self.CharacterMovement`))
  (bind _asanimal_state (cast `/Game/AnimalGuys/2_JungGuJin/GameMode/AnimalState` (`self.PlayerState`)))
  (set `/Game/AnimalGuys/2_JungGuJin/GameMode/AnimalState.MaxMP` MaxMP _asanimal_state)
  (set `self.AttackCoolTime` AttackCoolTime)
  (set `self.MP_UseSizeOfAttack` MP_UseSizeOfAttack)
  (set `self.GetMPSpeed` GetMPSpeed)
  (set `self.DownTimeLength` DownTimeLength))

(fn `DisableOwnerHat`
  (bind _equipedhat (`self.EquipedHat`))
  (`/Engine/EditorBlueprintResources/StandardMacros.IsValid` _equipedhat
    (:`Is Valid`
      (`self.SetOwner` _equipedhat null))))

(fn `Do Ragdoll`
  (if (`self.IsCanCrush`)
    (set `self.IsCanCrush` false)
    (`PrimitiveComponent.SetSimulatePhysics` (`self.Mesh`) true)
    (`/Engine/EditorBlueprintResources/ActorMacros.Switch Has Authority`
      (:`Authority`
        (`KismetSystemLibrary.K2_SetTimer` null "ResRevive" 2.0)))))

(fn `DoGetUp`
  (set `self.IsCanCrush` true)
  (`PrimitiveComponent.SetSimulatePhysics` (`self.Mesh`) false)
  (`SceneComponent.K2_AttachToComponent` (`self.Mesh`) (`self.CapsuleComponent`) "None" "KeepRelative" "KeepRelative" "KeepRelative" true)
  (`SceneComponent.K2_SetRelativeLocationAndRotation` (`self.Mesh`) (0.0 0.0 -49.0) (struct :`Yaw` -90.0) false false))

(fn `DoRevive`
  (`self.DoGetUp`)
  (`/Engine/EditorBlueprintResources/ActorMacros.Switch Has Authority`
    (:`Authority`
      ;[1 1 1] 리스폰 장소 설정
      (bind _returnvalue (`GameplayStatics.GetActorOfClass` "/Game/AnimalGuys/2_JungGuJin/Blueprint/PlayerRevivePoint.PlayerRevivePoint_C"))
      (`self.K2_SetActorLocationAndRotation` (`self.K2_GetActorLocation` _returnvalue) (`self.K2_GetActorRotation` _returnvalue)))))

(fn `EnableOwnerHat`
  (params (EquipHat :type "Actor Object Reference"))
  (`self.SetOwner` (`self.GetController`)))

(fn `GetNearestHat`
  (returns (NesrestHat :type "Actor Object Reference"))
  (locals (NearestActor :type "Actor Object Reference") (NearestDist :type "Float (double-precision)" :default 122222.0))
  (for _array_element (`PrimitiveComponent.GetOverlappingActors` (`self.CapsuleComponent`) "/Game/AnimalGuys/2_JungGuJin/Cloth/Hat/HatParent/BP_Hat.BP_Hat_C")
    (if (`KismetSystemLibrary.DoesImplementInterface` _array_element "/Game/AnimalGuys/2_JungGuJin/Cloth/Hat/BPI_Cloth.BPI_Cloth_C")
      (bind _returnvalue (`KismetMathLibrary.Vector_Distance` (`self.K2_GetActorLocation`) (`self.K2_GetActorLocation` _array_element)))
      (if (> (`local.NearestDist`) _returnvalue)
        (set `local.NearestDist` _returnvalue)
        (set `local.NearestActor` _array_element))))
  (return (`local.NearestActor`)))

(fn `OnRep_Attack`
  (`self.SetAttack` (`self.Attack`)))

(fn `OnRep_Slide`
  (if (not (`self.IsInLobby?`))
    (`self.SetSlide` (`self.Slide`))))

(fn `SetAttack`
  (params (Attack :type Boolean))
  (if Attack
    (bind _asanimal_state (cast `/Game/AnimalGuys/2_JungGuJin/GameMode/AnimalState` (`self.PlayerState`)))
    (if (> (`/Game/AnimalGuys/2_JungGuJin/GameMode/AnimalState.CurMP` _asanimal_state) (`KismetMathLibrary.Conv_IntToDouble` (`self.MP_UseSizeOfAttack`)))
      (set `self.IsAttack` true))))

(fn `SetSlide`
  (params (Slide :type Boolean))
  (bind _defaultslidespeed (`self.DefaultSlideSpeed`))
  (if Slide
    (if (`self.CanSlide`)
      (set `self.IsSlide` true)
      (set `CharacterMovementComponent.MaxWalkSpeed` _defaultslidespeed (`self.CharacterMovement`))
      (set `self.DecressSlideSpeed` _defaultslidespeed))
    (else
      (set `self.IsSlide` false)
      (set `CharacterMovementComponent.MaxWalkSpeed` (`self.RunSpeed`) (`self.CharacterMovement`)))))

(fn `UserConstructionScript`)