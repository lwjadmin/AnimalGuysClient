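; BP_Hat is a hat that can be worn by a character or left loose as a physics object.
; AttachHat records the wearer, turns off the mesh's physics and collision, and snaps it to the character mesh's SKT_Hat socket, keeping world scale.
; DetachHat clears the wearer, restores collision and physics, and detaches the mesh in place.
; AttachCloth and DetachCloth are empty stubs here.
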(fn `AttachCloth`
  (params (Charactor :type "Character Object Reference"))
  (returns (Result :type Boolean))
  (return false))

(fn `AttachHat`
  (params (Charactor :type "Character Object Reference"))
  (returns (Result :type Boolean))
  (bind _staticmesh (`self.StaticMesh`))
  (set `self.OwnCharacter` Charactor)
  (`PrimitiveComponent.SetSimulatePhysics` _staticmesh false)
  (`PrimitiveComponent.SetCollisionEnabled` _staticmesh "NoCollision")
  (`self.K2_AttachToComponent` (`Character.Mesh` Charactor) "SKT_Hat" "SnapToTarget" "SnapToTarget" "KeepWorld")
  (return false))

(fn `DetachCloth`
  (returns (Result :type Boolean))
  (return false))

(fn `DetachHat`
  (returns (Result :type Boolean))
  (bind _staticmesh (`self.StaticMesh`))
  (set `self.OwnCharacter` null)
  (`PrimitiveComponent.SetCollisionEnabled` _staticmesh "QueryAndPhysics")
  (`PrimitiveComponent.SetSimulatePhysics` _staticmesh true)
  (`SceneComponent.K2_DetachFromComponent` (`self.StaticMesh`) "KeepWorld" "KeepWorld" "KeepWorld" true)
  (return false))

(fn `UserConstructionScript`)