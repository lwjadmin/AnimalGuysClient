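; Game mode for the AnimalGuys match that handles player joins, spawn placement and removal of the waiting wall.
; Each new player updates the current and remaining player counts on BP_AnimalGuys_GameState, and ChoosePlayerStart hands out PlayerStarts by incrementing index.
; BeginPlay caches the BP_WaitingBlock actor once the game state is valid.
; CallBreakWaitingWall starts a Tick-driven countdown that destroys that block after WaitingTime.
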(event `self.K2_PostLogin`
  (params (NewPlayer :type "PlayerController Object Reference"))
  ;[1 1 1] Event Handle Starting New Player와 유사하게 작동함[사용하지 않음]
)

(event `self.ReceiveBeginPlay`
  (`self.PrepareStart`))

(event `self.HandleStartingNewPlayer`
  (params (NewPlayer :type "PlayerController Object Reference"))
  (`parent.HandleStartingNewPlayer` NewPlayer)
  (bind _returnvalue (`self.GetNumPlayers`))
  (bind _asbp_animal_guys_game_state (cast `/Game/AnimalGuys/2_JungGuJin/GameMode/BP_AnimalGuys_GameState` (`GameplayStatics.GetGameState`)))
  (`/Game/AnimalGuys/2_JungGuJin/GameMode/BP_AnimalGuys_GameState.SetCurPlayerCount` _asbp_animal_guys_game_state _returnvalue)
  (`/Game/AnimalGuys/2_JungGuJin/GameMode/BP_AnimalGuys_GameState.SetLeftPlayerCount` _asbp_animal_guys_game_state _returnvalue))

(event `self.ReceiveTick`
  (params (DeltaSeconds :type "Float (single-precision)"))
  (bind _waitingblock (`self.WaitingBlock`))
  (if (`self.bBreakWallCall`)
    (bind _output_get (set `self.ElapsedTime` (+ DeltaSeconds (`self.ElapsedTime`))))
    (if (> _output_get (`self.WaitingTime`))
      (set `self.bBreakWallCall` false)
      (`/Engine/EditorBlueprintResources/StandardMacros.IsValid` _waitingblock
        (:`Is Valid`
          (`self.K2_DestroyActor` _waitingblock))))))

(fn `CallBreakWaitingWall`
  (set `self.bBreakWallCall` true)
  (set `self.ElapsedTime` 0.0))

(fn `ChoosePlayerStart`
  (params (Player :type "Controller Object Reference"))
  (returns (ReturnValue :type "Actor Object Reference"))
  (locals (TempActor :type "Actor Object Reference"))
  (bind _outactors (`GameplayStatics.GetAllActorsOfClass` "/Script/Engine.PlayerStart"))
  (bind _output_get (set `local.TempActor` (`|GetArrayItem` _outactors (`self.PlayerStartIdx`))))
  (`/Engine/EditorBlueprintResources/StandardMacros.IncrementInt` (`self.PlayerStartIdx`)
    (:`  `
      (return _output_get))))

(fn `PrepareStart`
  (cast `/Game/AnimalGuys/2_JungGuJin/GameMode/BP_AnimalGuys_GameState` (`GameplayStatics.GetGameState`)
    (:`then`
      (bind _returnvalue (`GameplayStatics.GetActorOfClass` "/Game/AnimalGuys/Combined/Blueprints/GamePlay/BP_WaitingBlock.BP_WaitingBlock_C"))
      (`/Engine/EditorBlueprintResources/StandardMacros.IsValid` _returnvalue
        (:`Is Valid`
          (set `self.WaitingBlock` _returnvalue))))
    (:`CastFailed`
      (`KismetSystemLibrary.K2_SetTimer` null "PrepareStart"))))

(fn `UserConstructionScript`)