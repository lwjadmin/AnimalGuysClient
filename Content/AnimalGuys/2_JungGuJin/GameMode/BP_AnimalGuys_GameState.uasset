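; Game state for Animal Guys that tracks player counts and places characters when a game finishes.
; Current, left and game player counts use RepNotify to broadcast update dispatchers, with debug prints for the first two.
; BeginPlay sets a default game player count, then overrides it from the session's SessionGamePlayer setting if found.
; ProcessFinish moves winners and losers to random locations inside the winner and loser area actors.
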(event `self.ReceiveBeginPlay`
  (`|ExecutionSequence`
    (:`then_0`
      (`self.SetGamePlayerCount` 2))
    (:`then_1`
      (bind (_numconnections _numprivateconnections _bislan _bisdedicated _ballowinvites _ballowjoininprogress _bisanticheatenabled _builduniqueid _extrasettings) (`AdvancedSessionsLibrary.GetSessionSettings`)
        (:`OnSuccess`
          (`KismetSystemLibrary.PrintString` "SessionLoad Success")
          (bind _settingvalue (`AdvancedSessionsLibrary.GetSessionPropertyInt` _extrasettings "SessionGamePlayer")
            (:`Found`
              (`self.SetGamePlayerCount` _settingvalue))))
        (:`OnFailure`
          (`KismetSystemLibrary.PrintString` "SessionLoad Fail"))))))

(fn `OnRep_CurPlayerCount`
  (bind _curplayercount (`self.CurPlayerCount`))
  (`self.EventDispatcher_UpdateCurPlayerCount` _curplayercount)
  (`KismetSystemLibrary.PrintString` (`KismetStringLibrary.Concat_StrStr` "CurPlayerCount : " (`KismetStringLibrary.Conv_IntToString` _curplayercount)) true true (struct :`G` 0.66 :`B` 1.0 :`A` 1.0) 600.0))

(fn `OnRep_GamePlayerCount`
  (`self.EventDispatcher_UpdateGamePlayerCount` (`self.GamePlayerCount`)))

(fn `OnRep_LeftPlayerCount`
  (bind _leftplayercount (`self.LeftPlayerCount`))
  (`self.EventDispatcher_UpdateLeftPlayerCount` _leftplayercount)
  (`KismetSystemLibrary.PrintString` (`KismetStringLibrary.Concat_StrStr` "LeftPlayerCount : " (`KismetStringLibrary.Conv_IntToString` _leftplayercount)) true true (struct :`G` 0.66 :`B` 1.0 :`A` 1.0) 600.0))

(fn `ProcessFinish`
  (params (WinnerCharArray :type "Array of /Game/AnimalGuys/2_JungGuJin/Character/BP_AnimalGuys_Character Object Reference") (LoserCharArray :type "Array of /Game/AnimalGuys/2_JungGuJin/Character/BP_AnimalGuys_Character Object Reference"))
  (for _array_element WinnerCharArray
    (bind _returnvalue (`GameplayStatics.GetActorOfClass` "/Game/AnimalGuys/3_KangHoJae/Levels/GamePlay/Blueprint/BPA_WinnerArea.BPA_WinnerArea_C"))
    (`/Engine/EditorBlueprintResources/StandardMacros.IsValid` _returnvalue
      (:`Is Valid`
        (bind _outlocation (`/Game/AnimalGuys/3_KangHoJae/Levels/GamePlay/Blueprint/BPA_WinnerArea.GetRandomLocationInArea` _returnvalue))
        (`self.K2_SetActorLocation` _array_element _outlocation false false))))
  (for _array_element_2 LoserCharArray
    (bind _returnvalue_2 (`GameplayStatics.GetActorOfClass` "/Game/AnimalGuys/3_KangHoJae/Levels/GamePlay/Blueprint/BPA_LoserArea.BPA_LoserArea_C"))
    (`/Engine/EditorBlueprintResources/StandardMacros.IsValid` _returnvalue_2
      (:`Is Valid`
        (bind _outlocation_2 (`/Game/AnimalGuys/3_KangHoJae/Levels/GamePlay/Blueprint/BPA_LoserArea.GetRandomLocationInArea` _returnvalue_2))
        (`self.K2_SetActorLocation` _array_element_2 _outlocation_2 false false)))))

(fn `SetCurPlayerCount`
  (params (CurPlayerCount :type Integer))
  (set `self.CurPlayerCount` CurPlayerCount))

(fn `SetGamePlayerCount`
  (params (GamePlayerCount :type Integer))
  (set `self.GamePlayerCount` GamePlayerCount))

(fn `SetLeftPlayerCount`
  (params (LeftPlayerCount :type Integer))
  (set `self.LeftPlayerCount` LeftPlayerCount))

(fn `UserConstructionScript`)