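; Player state for AnimalGuys that holds each player's MP, animal type and clothing choice.
; MP functions spend or restore a clamped value and report depletion or recovery past a threshold, while its RepNotify broadcasts changes through a dispatcher.
; Animal and clothing RepNotifies call the matching appearance change on the owning character.
; OnDamaged flags player character 0 as damaged, rather than this state's own pawn.
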(fn `Get MP_Slide`
  (params (GetRest :type "Float (double-precision)"))
  (returns (IsMor20 :type Boolean))
  (bind _output_get (set `self.CurMP` (`KismetMathLibrary.FClamp` (+ (`self.CurMP`) GetRest) 0.0 (`self.MaxMP`))))
  (return (> _output_get 20.0)))

(fn `IsCanUseMP`
  (returns (IsNull :type Boolean))
  (return (<= (`self.CurMP`) 0.0)))

(fn `On Damaged`
  (bind _asbp_animal_guys (cast `/Game/AnimalGuys/2_JungGuJin/Character/BP_AnimalGuys_Character` (`GameplayStatics.GetPlayerCharacter` 0)))
  (set `/Game/AnimalGuys/2_JungGuJin/Character/BP_AnimalGuys_Character.IsDamaged` true _asbp_animal_guys))

(fn `OnRep_AnimalType`
  (cast `/Game/AnimalGuys/2_JungGuJin/Character/BP_AnimalGuys_Character` (`self.PawnPrivate`))
  (switch `int` (`self.AnimalType`)
    (:`0`
      (`self.ChangeKitty`))
    (:`1`
      (`self.ChangePiggy`))
    (:`2`
      (`self.ChangeDoggy`))
    (:`3`
      (`self.ChangeBunny`))))

(fn `OnRep_ClothColor`
  (cast `/Game/AnimalGuys/2_JungGuJin/Character/BP_AnimalGuys_Character` (`self.PawnPrivate`))
  (switch `int` (`self.ClothType`)
    (:`0`
      (`self.ChangeBared`))
    (:`1`
      (`self.ChaneA`))
    (:`2`
      (`self.ChangeB`))
    (:`3`
      (`self.ChangeC`))))

(fn `OnRep_CurMP`
  (`self.NewEventDispatcher_ChangeMP` (`self.CurMP`) (`self.MaxMP`)))

(fn `SetAnimalType`
  (params (AnimalType :type Integer))
  (set `self.AnimalType` AnimalType))

(fn `SetCloth`
  (params (ClothType :type Integer))
  (set `self.ClothType` ClothType))

(fn `UseMP_Slide`
  (params (TrySlide :type "Float (double-precision)"))
  (returns (IsNull :type Boolean))
  (bind _output_get (set `self.CurMP` (`KismetMathLibrary.FClamp` (- (`self.CurMP`) TrySlide) 0.0 (`self.MaxMP`))))
  (return (<= _output_get 0.0)))

(fn `UseMPAttack`
  (params (B :type "Float (double-precision)"))
  (returns (IsNull :type Boolean))
  (bind _output_get (set `self.CurMP` (`KismetMathLibrary.FClamp` (- (`self.CurMP`) B) 0.0 (`self.MaxMP`))))
  (return (<= _output_get 0.0)))

(fn `UserConstructionScript`)