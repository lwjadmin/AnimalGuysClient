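; AnimalGuys HUD that shows the local player's MP and current player count in a widget and presents the win/lose reward screen.
; On BeginPlay it creates the widget, then retries on a timer until it can bind to the PlayerState's MP-change dispatcher.
; Player count updates through an OnRep, and the reward screen switches input to UI-only.
; Finishing the game destroys the session on authority or logs out remotely, returning to the session level on success.
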(event `self.ReceiveBeginPlay`
  (bind _returnvalue (`GameplayStatics.GetPlayerController` 0))
  (bind _returnvalue_2 (`|CreateWidget` "/Game/AnimalGuys/2_JungGuJin/Widget/UMG_AnimalGuys_HudWidget.UMG_AnimalGuys_HudWidget_C"))
  (bind _output_get (set `self.AnimalHudWidget` _returnvalue_2))
  (`UserWidget.AddToViewport` _output_get 0)
  (`WidgetBlueprintLibrary.SetInputMode_GameOnly` _returnvalue)
  (set `PlayerController.bShowMouseCursor` false _returnvalue)
  (`self.BindPlayerState`))

(event `EventOnClick_FinishGame`
  (`/Engine/EditorBlueprintResources/ActorMacros.Switch Has Authority`
    (:`Authority`
      (`DestroySessionCallbackProxy.DestroySession` (`GameplayStatics.GetPlayerController` 0)
        (:`OnSuccess`
          _)))
    (:`Remote`
      (`LogoutUserCallbackProxy.LogoutUser` (`GameplayStatics.GetPlayerController` 0)
        (:`OnSuccess`
          _))))
  (`GameplayStatics.OpenLevel` "AnimalGuys_CreateJoinSessionLevel"))

(fn `BindPlayerState`
  (bind _asbp_animal_guys_player_state (cast `/Game/AnimalGuys/2_JungGuJin/GameMode/BP_AnimalGuys_PlayerState` (`Controller.PlayerState` (`GameplayStatics.GetPlayerController` 0)))
    (:`then`
      (add `/Game/AnimalGuys/2_JungGuJin/GameMode/BP_AnimalGuys_PlayerState.NewEventDispatcher_ChangeMP` _asbp_animal_guys_player_state (`|CreateDelegate` :!event `UpdateMyMP`))
      (`self.UpdateMyMP` (`/Game/AnimalGuys/2_JungGuJin/GameMode/BP_AnimalGuys_PlayerState.CurMP` _asbp_animal_guys_player_state) (`/Game/AnimalGuys/2_JungGuJin/GameMode/BP_AnimalGuys_PlayerState.MaxMP` _asbp_animal_guys_player_state)))
    (:`CastFailed`
      (`KismetSystemLibrary.K2_SetTimer` null "BindPlayerState" 0.1))))

(fn `OnRep_CurPlayerCount`
  (bind _animalhudwidget (`self.AnimalHudWidget`))
  (`/Engine/EditorBlueprintResources/StandardMacros.IsValid` _animalhudwidget
    (:`Is Valid`
      (`/Game/AnimalGuys/2_JungGuJin/Widget/UMG_AnimalGuys_HudWidget.SetCurPlayerCount` _animalhudwidget (`self.CurPlayerCount`)))))

(fn `ShowRewardWidget`
  (params (WinnerActor :type "Array of Actor Object Reference"))
  (bind _returnvalue (`GameplayStatics.GetPlayerController` 0))
  (bind _returnvalue_2 (`|CreateWidget` "/Game/AnimalGuys/1_LeeWoongJae/Widget/UMG_RewardWidget.UMG_RewardWidget_C" null (>= (`KismetArrayLibrary.Array_Find` WinnerActor (`GameplayStatics.GetPlayerCharacter` 0)) 0)))
  (bind _output_get (set `self.RewardWidget` _returnvalue_2))
  (`UserWidget.AddToViewport` _output_get 0)
  (`WidgetBlueprintLibrary.SetInputMode_UIOnlyEx` _returnvalue _output_get)
  (set `PlayerController.bShowMouseCursor` true _returnvalue))

(fn `UpdateMyMP`
  (params (CurMP :type "Float (double-precision)") (MaxMP :type "Float (double-precision)"))
  (bind _animalhudwidget (`self.AnimalHUDWidget`))
  (`/Engine/EditorBlueprintResources/StandardMacros.IsValid` _animalhudwidget
    (:`Is Valid`
      (`/Game/AnimalGuys/2_JungGuJin/Widget/UMG_AnimalGuys_HudWidget.SetMP` _animalhudwidget CurMP MaxMP))))

(fn `UserConstructionScript`)