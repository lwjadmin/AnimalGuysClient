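; Spinner obstacle that rotates continuously and damages animal characters that collide with it.
; Each tick it resets the spinner mesh's world rotation to yaw only, then adds local yaw scaled by SpinnerSpeed and delta time.
; Mesh hits call ReqCrash, which applies damage to BP_AnimalBaseOrigin actors.
; The Reqdd and Resdd events are empty, unused stubs.
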(event `Resdd`)

(event `Reqdd`
  (`self.Resdd`))

(event `self.ReceiveTick`
  (params (DeltaSeconds :type "Float (single-precision)"))
  (bind _sm_spinner_v1 (`self.SM_Spinner_V1`))
  (bind (_returnvalue_roll _returnvalue_pitch _returnvalue_yaw) (`KismetMathLibrary.BreakRotator` (`SceneComponent.K2_GetComponentRotation` _sm_spinner_v1)))
  (bind _output_get (set `self.Return Value Z (Yaw)` _returnvalue_yaw))
  (`SceneComponent.K2_SetWorldRotation` (`self.SM_Spinner_V1`) (`KismetMathLibrary.MakeRotator` 0.0 0.0 _output_get) false false)
  (`SceneComponent.K2_AddLocalRotation` _sm_spinner_v1 (`KismetMathLibrary.MakeRotator` 0.0 0.0 (* DeltaSeconds (`self.SpinnerSpeed`))) false false))

(event `self.SM_Spinner_V1.OnComponentHit`
  (params (HitComponent :type "PrimitiveComponent Object Reference") (OtherActor :type "Actor Object Reference") (OtherComp :type "PrimitiveComponent Object Reference") (NormalImpulse :type "Vector Structure") (Hit :type "HitResult Structure (by ref)"))
  ;[1 1 1] ApplyDamage to Character
  (`self.ReqCrash`))

(event `ReqCrash`
  ;[1 1 1] ApplyDamage to Character
  (bind _asbp_animal_base_origin (cast `/Game/AnimalGuys/2_JungGuJin/Character/CharacterBase/BP_AnimalBaseOrigin` (stale `self.SM_Spinner_V1.OnComponentHit` OtherActor)))
  (`GameplayStatics.ApplyDamage` _asbp_animal_base_origin 1.0 null self))

(fn `UserConstructionScript`)