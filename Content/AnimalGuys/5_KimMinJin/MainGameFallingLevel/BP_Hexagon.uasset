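; BP_Hexagon is a hexagon tile in the falling level that disappears shortly after being touched.
; On BeginPlay it gives its static mesh a random material from the RandomMaterial array.
; The first overlap of its Box, with no filter on the overlapping actor, nudges the tile down and swaps in TouchedMaterial.
; A DoOnce blocks repeat triggers, and the actor destroys itself after a short delay.
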(event `self.ReceiveBeginPlay`
  (`PrimitiveComponent.SetMaterial` (`self.StaticMesh`) 0 (`KismetArrayLibrary.Array_Random` (`self.RandomMaterial`))))

(event `self.Box.OnComponentBeginOverlap`
  (params (OverlappedComponent :type "PrimitiveComponent Object Reference") (OtherActor :type "Actor Object Reference") (OtherComp :type "PrimitiveComponent Object Reference") (OtherBodyIndex :type Integer) (bFromSweep :type Boolean) (SweepResult :type "HitResult Structure (by ref)"))
  (`/Engine/EditorBlueprintResources/StandardMacros.DoOnce` false
    (:`Completed`
      (`self.K2_AddActorLocalOffset` (0.0 0.0 -10.0))
      (`PrimitiveComponent.SetMaterial` (`self.StaticMesh`) 0 (`self.TouchedMaterial`))
      (`KismetSystemLibrary.Delay` 1.0)
      (`self.K2_DestroyActor`))))

(fn `UserConstructionScript`)