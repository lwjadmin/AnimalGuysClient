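; BP_MJ_SlidingEffect is a one-shot slip hazard that spins an AnimalGuys character who touches its mesh.
; The first character overlap only arms it and records that controller; the controller comparison on later overlaps leads to the same result either way.
; A later overlap disables input for player controller 0 and applies timeline-driven yaw rotation to the character.
; After a short delay it restores input and destroys itself.
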(event `self.StaticMesh.OnComponentBeginOverlap`
  (params (OverlappedComponent :type "PrimitiveComponent Object Reference") (OtherActor :type "Actor Object Reference") (OtherComp :type "PrimitiveComponent Object Reference") (OtherBodyIndex :type Integer) (bFromSweep :type Boolean) (SweepResult :type "HitResult Structure (by ref)"))
  (bind _asbp_animal_guys_character (cast `/Game/AnimalGuys/2_JungGuJin/Character/BP_AnimalGuys_Character` OtherActor))
  (if (`self.IsOverlapOnce`)
    (if (!= (`Pawn.GetController` _asbp_animal_guys_character) (stale _output_get))
      _
      (else
        _))
    (`self.DisableInput` _asbp_animal_guys_character (`GameplayStatics.GetPlayerController` 0))
    (bind (_direction `_새_트랙_0`) (`Timeline|타임라인_0`)
      (:`Update`
        (`self.K2_AddActorLocalRotation` _asbp_animal_guys_character (`KismetMathLibrary.MakeRotator` 0.0 0.0 `_새_트랙_0`) false false))
      (:`Finished`
        (`KismetSystemLibrary.Delay` 2.0)
        (`self.EnableInput` _asbp_animal_guys_character (`GameplayStatics.GetPlayerController` 0))
        (`self.K2_DestroyActor`)))
    (else
      (set `self.IsOverlapOnce` true)
      (bind _output_get (set `self.controller` (`Pawn.GetController` _asbp_animal_guys_character))))))

(event `self.StaticMesh.OnComponentEndOverlap`
  (params (OverlappedComponent :type "PrimitiveComponent Object Reference") (OtherActor :type "Actor Object Reference") (OtherComp :type "PrimitiveComponent Object Reference") (OtherBodyIndex :type Integer))
  (bind _asbp_animal_guys_character (cast `/Game/AnimalGuys/2_JungGuJin/Character/BP_AnimalGuys_Character` OtherActor))
  (set `self.As BP Animal Guys Character` _asbp_animal_guys_character))

(fn `UserConstructionScript`)