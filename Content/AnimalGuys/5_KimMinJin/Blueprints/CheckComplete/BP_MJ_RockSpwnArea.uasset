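; Rock-spawning trigger area that sends out falling rocks when an AnimalGuys character overlaps its cube.
; Overlap runs a looping SpawnArea timer for ten seconds; BeginPlay caches the last TargetPoint found with the configured tag.
; Each tick of the timer spawns a BP_MJ_FallingRocks at a random spot around that point, gated on a character controlled by player controller 0.
; The physics impulse logic for the rocks is disconnected.
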(event `self.Cube.OnComponentBeginOverlap`
  (params (OverlappedComponent :type "PrimitiveComponent Object Reference") (OtherActor :type "Actor Object Reference") (OtherComp :type "PrimitiveComponent Object Reference") (OtherBodyIndex :type Integer) (bFromSweep :type Boolean) (SweepResult :type "HitResult Structure (by ref)"))
  (cast `/Game/AnimalGuys/2_JungGuJin/Character/BP_AnimalGuys_Character` OtherActor)
  (`KismetSystemLibrary.K2_SetTimer` null "SpawnArea" 0.7 true)
  (`KismetSystemLibrary.Delay` 10.0)
  (`KismetSystemLibrary.K2_ClearTimer` null "SpawnArea"))

(event `self.ReceiveBeginPlay`
  (bind _outactors (`GameplayStatics.GetAllActorsOfClassWithTag` "/Script/Engine.TargetPoint" (`self.Tag`)))
  (for _array_element _outactors
    (set `self.RocksTargetPoint` _array_element)))

(fn `SpawnArea`
  (bind _rockstargetpoint (`self.RocksTargetPoint`))
  (bind _outactors (`GameplayStatics.GetAllActorsOfClass` "/Game/AnimalGuys/2_JungGuJin/Character/BP_AnimalGuys_Character.BP_AnimalGuys_Character_C"))
  (for _array_element _outactors
    (if (== (`Pawn.GetController` _array_element) (`GameplayStatics.GetPlayerController` 0))
      (bind _returnvalue (`|SpawnActorFromClass` "/Game/AnimalGuys/5_KimMinJin/Blueprints/CheckComplete/BP_MJ_FallingRocks.BP_MJ_FallingRocks_C" (`KismetMathLibrary.MakeTransform` (`KismetMathLibrary.RandomPointInBoundingBox` (`self.K2_GetActorLocation` _rockstargetpoint) (0.0 200.0 200.0)) (`self.K2_GetActorRotation` _rockstargetpoint)) "Undefined" "OverrideRootScale" null null))
      (bind _output_get (set `self.FallingRocks` _returnvalue)))))

(fn `UserConstructionScript`)