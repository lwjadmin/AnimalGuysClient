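; BP_WoodGun is an automatic turret actor that rotates and periodically fires wooden bullets.
; A timeline started on BeginPlay drives the actor's yaw rotation.
; Tick accumulates elapsed time and, every few seconds, spawns a BP_WoodBullet at the Arrow component's world transform.
; The RepeatRotate function only calls SetActorRotation with no inputs and is not called within this Blueprint.
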(event `self.ReceiveBeginPlay`
  (bind (_direction _angle) (`Timeline|타임라인_0`)
    (:`Update`
      (`self.K2_SetActorRotation` (`KismetMathLibrary.MakeRotator` 0.0 0.0 _angle)))))

(event `self.ReceiveTick`
  (params (DeltaSeconds :type "Float (single-precision)"))
  (bind _output_get (set `self.ElapsedTime` (+ (`self.ElapsedTime`) DeltaSeconds)))
  (if (> _output_get 3.0)
    (set `self.ElapsedTime` 0.0)
    (`|SpawnActorFromClass` "/Game/AnimalGuys/5_KimMinJin/Blueprints/CheckComplete/BP_WoodBullet.BP_WoodBullet_C" (`SceneComponent.K2_GetComponentToWorld` (`self.Arrow`)) "Undefined" "OverrideRootScale" null null)))

(fn `RepeatRotate`
  (`self.K2_SetActorRotation` (`KismetMathLibrary.MakeRotator` 0.0)))

(fn `UserConstructionScript`)