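; BP_MJ_SpawnItem is an item spawner that keeps a random effect item at its own location, drawn from size, jump, sliding and speed effects.
; On BeginPlay it fills the class array and spawns a random pick at the actor's transform.
; A BoxCollision overlap destroys the live item and sets a flag.
; Tick then accumulates time and spawns a new random item once three seconds have passed.
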(event `self.ReceiveBeginPlay`
  (bind _output_get (set `self.ItemArray` (`|MakeArray` "/Game/AnimalGuys/5_KimMinJin/Blueprints/CheckComplete/BP_SmallerEffect.BP_SmallerEffect_C" "/Game/AnimalGuys/5_KimMinJin/Blueprints/CheckComplete/BP_TallEffect.BP_TallEffect_C" "/Game/AnimalGuys/5_KimMinJin/Blueprints/CheckComplete/BP_JumpHigher.BP_JumpHigher_C" "/Game/AnimalGuys/5_KimMinJin/Blueprints/CheckComplete/BP_JumpLower.BP_JumpLower_C" "/Game/AnimalGuys/5_KimMinJin/Blueprints/CheckComplete/BP_MJ_SlidingEffect.BP_MJ_SlidingEffect_C" "/Game/AnimalGuys/5_KimMinJin/Blueprints/CheckComplete/BP_SlowDown.BP_SlowDown_C" "/Game/AnimalGuys/5_KimMinJin/Blueprints/CheckComplete/BP_SpeedBoost.BP_SpeedBoost_C" :!type "Actor Class Reference")))
  (bind _returnvalue (`|SpawnActorFromClass` (`KismetArrayLibrary.Array_Random` _output_get) (`self.GetTransform`) "Undefined" "OverrideRootScale" null null))
  (set `self.SpawnItem` _returnvalue))

(event `self.BoxCollision.OnComponentBeginOverlap`
  (params (OverlappedComponent :type "PrimitiveComponent Object Reference") (OtherActor :type "Actor Object Reference") (OtherComp :type "PrimitiveComponent Object Reference") (OtherBodyIndex :type Integer) (bFromSweep :type Boolean) (SweepResult :type "HitResult Structure (by ref)"))
  (bind _spawnitem (`self.SpawnItem`))
  (`/Engine/EditorBlueprintResources/StandardMacros.IsValid` _spawnitem
    (:`Is Valid`
      (`self.K2_DestroyActor` _spawnitem)
      (set `self.bItemDestroyed` true))))

(event `self.ReceiveTick`
  (params (DeltaSeconds :type "Float (single-precision)"))
  (if (`self.bItemDestroyed`)
    (bind _output_get (set `self.ElapsedTime` (+ DeltaSeconds (`self.ElapsedTime`))))
    (if (> _output_get 3.0)
      (bind _returnvalue (`|SpawnActorFromClass` (`KismetArrayLibrary.Array_Random` (`self.ItemArray`)) (`self.GetTransform`) "Undefined" "OverrideRootScale" null null))
      (set `self.SpawnItem` _returnvalue)
      (set `self.bItemDestroyed` false)
      (set `self.ElapsedTime` 0.0))))

(fn `UserConstructionScript`)