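; BP_MJ_FallingRocks is a short-lived falling rock hazard that damages actors it hits.
; On BeginPlay, the authority picks a random mesh, indexes the scale array with a random pick that may not match it, and sets a three-second lifespan.
; Authority applies damage on mesh hits, while overlap by the first player's character spawns another rock at the mesh's transform.
; Physics knockback and launch logic remain unconnected.
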(event `self.ReceiveBeginPlay`
  (bind _staticmesh (`self.StaticMesh`))
  (bind (_outitem _outindex) (`KismetArrayLibrary.Array_Random` (`self.NewVar_0`)))
  (`/Engine/EditorBlueprintResources/ActorMacros.Switch Has Authority`
    (:`Authority`
      (`StaticMeshComponent.SetStaticMesh` _staticmesh _outitem)
      (`SceneComponent.SetRelativeScale3D` _staticmesh (`|GetArrayItem` (`self.NewVar_1`) _outindex))
      (`self.SetLifeSpan` 3.0))))

(event `self.StaticMesh.OnComponentBeginOverlap`
  (params (OverlappedComponent :type "PrimitiveComponent Object Reference") (OtherActor :type "Actor Object Reference") (OtherComp :type "PrimitiveComponent Object Reference") (OtherBodyIndex :type Integer) (bFromSweep :type Boolean) (SweepResult :type "HitResult Structure (by ref)"))
  (bind _asbp_animal_guys_character (cast `/Game/AnimalGuys/2_JungGuJin/Character/BP_AnimalGuys_Character` OtherActor))
  (if (== (`Pawn.GetController` _asbp_animal_guys_character) (`GameplayStatics.GetPlayerController` 0))
    (bind _returnvalue (`|SpawnActorFromClass` "BP_MJ_FallingRocks_C" (`SceneComponent.GetSocketTransform` (`self.StaticMesh`) "None" "RTS_World") "Undefined" "OverrideRootScale" null null))))

(event `self.StaticMesh.OnComponentHit`
  (params (HitComponent :type "PrimitiveComponent Object Reference") (OtherActor :type "Actor Object Reference") (OtherComp :type "PrimitiveComponent Object Reference") (NormalImpulse :type "Vector Structure") (Hit :type "HitResult Structure (by ref)"))
  (`/Engine/EditorBlueprintResources/ActorMacros.Switch Has Authority`
    (:`Authority`
      (`GameplayStatics.ApplyDamage` OtherActor 1.0 null self))))

(fn `UserConstructionScript`)