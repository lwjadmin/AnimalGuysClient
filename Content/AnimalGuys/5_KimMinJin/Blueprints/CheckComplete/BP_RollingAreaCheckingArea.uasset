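; BP_RollingAreaCheckingArea is a trigger that launches a rolling obstacle when an AnimalGuys character overlaps its Cube.
; KABOOM loops over all characters and spawns a BP_RollingObject only for the one controlled by player controller 0, whichever character triggered it.
; The object appears at a random lateral and vertical offset around SpawnPoint, then gets physics and a strong forward impulse.
; Every overlap repeats the spawn, with no one-shot guard.
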(event `self.Cube.OnComponentBeginOverlap`
  (params (OverlappedComponent :type "PrimitiveComponent Object Reference") (OtherActor :type "Actor Object Reference") (OtherComp :type "PrimitiveComponent Object Reference") (OtherBodyIndex :type Integer) (bFromSweep :type Boolean) (SweepResult :type "HitResult Structure (by ref)"))
  (cast `/Game/AnimalGuys/2_JungGuJin/Character/BP_AnimalGuys_Character` OtherActor)
  (`self.KA_BOOM`))

(fn `KA_BOOM`
  (bind _spawnpoint (`self.SpawnPoint`))
  (bind _outactors (`GameplayStatics.GetAllActorsOfClass` "/Game/AnimalGuys/2_JungGuJin/Character/BP_AnimalGuys_Character.BP_AnimalGuys_Character_C"))
  (for _array_element _outactors
    (if (== (`Pawn.GetController` _array_element) (`GameplayStatics.GetPlayerController` 0))
      (bind _returnvalue (`|SpawnActorFromClass` "/Game/AnimalGuys/5_KimMinJin/Blueprints/CheckComplete/BP_RollingObject.BP_RollingObject_C" (`KismetMathLibrary.MakeTransform` (`KismetMathLibrary.RandomPointInBoundingBox` (`self.K2_GetActorLocation` _spawnpoint) (0.0 200.0 200.0)) (`self.K2_GetActorRotation` _spawnpoint)) "Undefined" "OverrideRootScale" null null))
      (bind _output_get (set `self.RollingObject` _returnvalue))
      (bind _staticmesh (`/Game/AnimalGuys/5_KimMinJin/Blueprints/CheckComplete/BP_RollingObject.StaticMesh` _output_get))
      (`PrimitiveComponent.SetSimulatePhysics` _staticmesh true)
      (`PrimitiveComponent.AddImpulse` _staticmesh (* (`SceneComponent.GetForwardVector` _staticmesh) 17000.0) "None" false))))

(fn `UserConstructionScript`)