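; BP_TCP is a network client actor that links the game to a TCP server and handles player sign-up messages.
; It connects on BeginPlay, optionally retries on a timer after disconnects, and shows connection state through its mesh material color.
; Received bytes are parsed into a four-integer header and dispatched by message ID to store socket IDs or report sign-up results.
; Outgoing sign-up requests pack that header with fixed-length ID, password and name fields.
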(event `self.ReceiveBeginPlay`
  (`self.NetConnect`))

(event `self.ReceiveDestroyed`
  (`self.Disconnect` (`self.NetConnectionID`)))

(event `self.ReceiveTick`
  (params (DeltaSeconds :type "Float (single-precision)"))
  (if (and (`self.DoReconnect`) (`|EnumEquality` (`self.NetworkState`) "NewEnumerator3"))
    (set `self.ElapsedSeconds` (+ (`self.ElapsedSeconds`) DeltaSeconds))
    (if (> (`self.ElapsedSeconds`) (`self.ReconnectIntervalSeconds`))
      (set `self.ElapsedSeconds` 0.0)
      (`self.NetConnect`))))

(fn `GetByteArrayWithoutRemoval`
  (params (InByteArray :type "Array of Byte") (StartIndex :type Integer) (ByteCount :type Integer))
  (returns (OutByteArray :type "Array of Byte"))
  (locals (TempByteArray :type "Array of Byte") (TempByteCount :type Integer))
  (set `local.TempByteCount` ByteCount)
  (for (_array_element _array_index) InByteArray
    (if (>= _array_index StartIndex)
      (`KismetArrayLibrary.Array_Add` (`local.TempByteArray`) _array_element)
      (bind _output_get (set `local.TempByteCount` (- (`local.TempByteCount`) 1)))
      (if (<= _output_get 0)
        (break))))
  (return (`local.TempByteArray`)))

(fn `GetMessageHeader`
  (params (InByteArray :type "Array of Byte"))
  (returns (OutByteArray :type "Array of Byte") (OutMessageHeader :type "/Game/AnimalGuys/1_LeeWoongJae/Network/ST_MessageHeader Structure"))
  (locals (TempMessageHeader :type "/Game/AnimalGuys/1_LeeWoongJae/Network/ST_MessageHeader Structure") (TempByteArray :type "Array of Byte"))
  (bind _output_get (set `local.TempByteArray` InByteArray))
  (bind _returnvalue (`self.Message_ReadInt` _output_get))
  (bind _returnvalue_2 (`self.Message_ReadInt` _output_get))
  (bind _returnvalue_3 (`self.Message_ReadInt` _output_get))
  (bind _returnvalue_4 (`self.Message_ReadInt` _output_get))
  (return _output_get (make `/Game/AnimalGuys/1_LeeWoongJae/Network/ST_MessageHeader` _returnvalue _returnvalue_2 _returnvalue_3 _returnvalue_4)))

(fn `MakeFixedStringByteArray`
  (params (InString :type String) (InFixedByteLength :type Integer))
  (returns (OutByteArray :type "Array of Byte") (OutMakeSuccess :type Boolean))
  (locals (TempByteArray :type "Array of Byte"))
  (bind _returnvalue (`self.Conv_StringToBytes` InString))
  (bind _returnvalue_2 (- InFixedByteLength (`KismetArrayLibrary.Array_Length` _returnvalue)))
  (if (>= _returnvalue_2 0)
    (`KismetArrayLibrary.Array_Resize` (`local.TempByteArray`) _returnvalue_2)
    (return (`self.Concat_BytesBytes` _returnvalue (`local.TempByteArray`)) true)
    (else
      (`KismetArrayLibrary.Array_Resize` (`local.TempByteArray`) InFixedByteLength)
      (return (`local.TempByteArray`) false))))

(fn `MakeMsgHeaderByteArray`
  (params (InMessageID :type Integer) (InMessageSize :type Integer) (InSenderSocketID :type Integer) (InReceiverSocketID :type Integer))
  (returns (OutByteArray :type "Array of Byte"))
  (return (`self.Concat_BytesBytes` (`self.Conv_IntToBytes` InMessageID) (`self.Conv_IntToBytes` InMessageSize) (`self.Conv_IntToBytes` InSenderSocketID) (`self.Conv_IntToBytes` InReceiverSocketID))))

(fn `NetConnect`
  (bind _connectionid (`self.Connect` (`self.NetServerAddress`) (`self.NetServerPort`) (`|CreateDelegate` :!event `NetDisconnectd`) (`|CreateDelegate` :!event `NetConnected`) (`|CreateDelegate` :!event `NetReceived`)))
  (set `self.NetConnectionID` _connectionid)
  (bind _output_get (set `self.NetworkState` "NewEnumerator1"))
  (`PrimitiveComponent.SetMaterial` (`self.StaticMesh`) 0 "/Game/AnimalGuys/1_LeeWoongJae/Network/MI_TCP_Orange.MI_TCP_Orange")
  (`KismetSystemLibrary.PrintString` (`|GetEnumeratorNameAsString` _output_get) true true (struct :`G` 0.66 :`B` 1.0 :`A` 1.0) 60.0))

(fn `NetConnected`
  (params (ConnectionId :type Integer))
  (set `self.NetConnectionID` ConnectionId)
  (bind _output_get (set `self.NetworkState` "NewEnumerator2"))
  (`PrimitiveComponent.SetMaterial` (`self.StaticMesh`) 0 "/Game/AnimalGuys/1_LeeWoongJae/Network/MI_TCP_Green.MI_TCP_Green")
  (`KismetSystemLibrary.PrintString` (`|GetEnumeratorNameAsString` _output_get) true true (struct :`G` 0.66 :`B` 1.0 :`A` 1.0) 60.0))

(fn `NetDisconnectd`
  (params (ConnectionId :type Integer))
  (`self.Disconnect` ConnectionId)
  (set `self.NetConnectionID` -1)
  (bind _output_get (set `self.NetworkState` "NewEnumerator3"))
  (`PrimitiveComponent.SetMaterial` (`self.StaticMesh`) 0 "/Game/AnimalGuys/1_LeeWoongJae/Network/MI_TCP_Red.MI_TCP_Red")
  (`KismetSystemLibrary.PrintString` (`|GetEnumeratorNameAsString` _output_get) true true (struct :`G` 0.66 :`B` 1.0 :`A` 1.0) 60.0))

(fn `NetProcessPacket`
  (params (InByteArray :type "Array of Byte"))
  (returns (Result :type "/Game/AnimalGuys/1_LeeWoongJae/Network/PacketProcessStatus Enum"))
  (locals (TempByteArray :type "Array of Byte") (NewLocalVar_0 :type "/Game/AnimalGuys/1_LeeWoongJae/Network/ST_MessageHeader Structure"))
  (bind _output_get (set `local.TempByteArray` InByteArray))
  (if (>= (`KismetArrayLibrary.Array_Length` _output_get) 16)
    (bind (_outbytearray _outmessageheader) (`self.GetMessageHeader` (`local.TempByteArray`)))
    (bind _output_get_2 (set `local.TempByteArray` _outbytearray))
    (bind (_messageid _messagesize _sendersocketid _receiversocketid) (break `/Game/AnimalGuys/1_LeeWoongJae/Network/ST_MessageHeader` _outmessageheader))
    (switch `int` _messageid
      (:`20001`
        (bind _result (`self.OnRecv_S2C_RES_CLIENT_CONNECT` _receiversocketid _sendersocketid))
        (return _result))
      (:`20003`
        (bind _result_2 (`self.OnRecv_S2C_RES_INSERT_PLAYER` _output_get_2))
        (return _result_2)))
    (else
      (return "NewEnumerator0"))))

(fn `NetReceived`
  (params (ConnectionId :type Integer) (Message :type "Array of Byte (by ref)"))
  (locals (RecvBuffer :type "Array of Byte") (RecvLength :type Integer))
  (if (== ConnectionId (`self.NetConnectionID`))
    (bind _output_get (set `local.RecvBuffer` Message))
    (set `local.RecvLength` (`KismetArrayLibrary.Array_Length` Message))
    (bind _result (`self.NetProcessPacket` _output_get))
    (switch `/Game/AnimalGuys/1_LeeWoongJae/Network/PacketProcessStatus` _result
      (:`NewEnumerator0`
        _)
      (:`NewEnumerator1`
        _)
      (:`NewEnumerator2`
        (`self.NetDisconnectd` (`self.NetConnectionID`))))
    (return)))

(fn `OnRecv_S2C_RES_CLIENT_CONNECT`
  (params (ClientSocketID :type Integer) (ServerSocketID :type Integer))
  (returns (Result :type "/Game/AnimalGuys/1_LeeWoongJae/Network/PacketProcessStatus Enum"))
  (`KismetSystemLibrary.PrintString` "S2C_RES_CLIENT_CONNECT CALLED" true true (struct :`G` 0.66 :`B` 1.0 :`A` 1.0) 60.0)
  (set `self.ClientSocketID` ClientSocketID)
  (set `self.ServerSocketID` ServerSocketID)
  (return "NewEnumerator1"))

(fn `OnRecv_S2C_RES_INSERT_PLAYER`
  (params (MsgBodyArray :type "Array of Byte"))
  (returns (Result :type "/Game/AnimalGuys/1_LeeWoongJae/Network/PacketProcessStatus Enum"))
  (locals (PlayerID :type String))
  (`KismetSystemLibrary.PrintString` "S2C_RES_INSERT_PLAYER CALLED" true true (struct :`G` 0.66 :`B` 1.0 :`A` 1.0) 60.0)
  (if (>= (`KismetArrayLibrary.Array_Length` MsgBodyArray) 30)
    (bind _returnvalue (`self.Message_ReadString` MsgBodyArray 30))
    (bind _output_get (set `local.PlayerID` _returnvalue))
    (if (`KismetStringLibrary.IsEmpty` _output_get)
      (`KismetSystemLibrary.PrintString` "회원가입 성공!" true true (struct :`G` 0.66 :`B` 1.0 :`A` 1.0) 60.0)
      (else
        (`KismetSystemLibrary.PrintString` "중복된 아이디가 존재합니다!" true true (struct :`G` 0.66 :`B` 1.0 :`A` 1.0) 60.0)))
    (return "NewEnumerator1")
    (else
      (return "NewEnumerator0"))))

(fn `OnSend_C2S_REQ_INSERT_PLAYER`
  (params (PlayerID :type String) (PlayerPWD :type String) (PlayerName :type String))
  (locals (MessagePacket :type "Array of Byte"))
  (`KismetSystemLibrary.PrintString` "C2S_REQ_INSERT_PLAYER CALLED" true true (struct :`G` 0.66 :`B` 1.0 :`A` 1.0) 60.0)
  (bind _outbytearray (`self.MakeMsgHeaderByteArray` 10001 (+ 12 30 30 30) (`self.ClientSocketID`) (`self.ServerSocketID`)))
  (bind _outbytearray_2 (`self.MakeFixedStringByteArray` PlayerID 30))
  (bind _outbytearray_3 (`self.MakeFixedStringByteArray` PlayerPWD 30))
  (bind _outbytearray_4 (`self.MakeFixedStringByteArray` PlayerName 30))
  (bind _returnvalue (`self.SendData` (`self.NetConnectionID`) (`self.Concat_BytesBytes` _outbytearray _outbytearray_2 _outbytearray_3 _outbytearray_4)))
  (if (not _returnvalue)
    (`self.NetDisconnectd` (`self.NetConnectionID`)))
  (return))

(fn `OverwriteByteArray`
  (params (InTargetByteArray :type "Array of Byte") (InByteArray :type "Array of Byte") (InStartIndex :type Integer))
  (returns (OutTargetByteArray :type "Array of Byte"))
  (bind _returnvalue (+ InStartIndex (`KismetArrayLibrary.Array_Length` InByteArray)))
  (if (> _returnvalue (`KismetArrayLibrary.Array_Length` InTargetByteArray))
    (return InTargetByteArray)
    (else
      (for _index (range InStartIndex (+ _returnvalue 1))
        (`KismetArrayLibrary.Array_Set` InTargetByteArray _index (`|GetArrayItem` InByteArray))))))

(fn `UserConstructionScript`)