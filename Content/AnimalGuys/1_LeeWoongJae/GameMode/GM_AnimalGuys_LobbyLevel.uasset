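; Lobby game mode for AnimalGuys that sends players back to the create/join session level.
; ReqMoveLevelExceptMe calls ResMoveLevelExceptMe, which opens that level directly.
; A separate MoveLevelExceptMe function, not called within this graph, loops over player controllers from index 1, skipping the first, and calls MoveLevel on each lobby HUD, stopping if a cast fails.
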(event `ReqMoveLevelExceptMe`
  (`self.ResMoveLevelExceptMe`))

(event `self.ReceiveBeginPlay`)

(event `ResMoveLevelExceptMe`
  (`GameplayStatics.OpenLevel` "AnimalGuys_CreateJoinSessionLevel"))

(fn `MoveLevelExceptMe`
  (bind _returnvalue (`self.GetNumPlayers`))
  (for _index (range 1 _returnvalue)
    (if true
      (bind _ashud_animal_guys_lobby_level (cast `/Game/AnimalGuys/1_LeeWoongJae/GameMode/HUD_AnimalGuys_LobbyLevel` (`PlayerController.GetHUD` (`GameplayStatics.GetPlayerController` _index))))
      (`/Game/AnimalGuys/1_LeeWoongJae/GameMode/HUD_AnimalGuys_LobbyLevel.MoveLevel` _ashud_animal_guys_lobby_level "AnimalGuys_CreateJoinSessionLevel"))))

(fn `UserConstructionScript`)