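; Lobby player controller for AnimalGuys that hands each player's locally stored profile over to the server.
; On possess, a client RPC reads the DB player info from the AnimalGuys game instance.
; It sends that data back through a server RPC, which stores the controller reference on the lobby PlayerState and applies the player info there.
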(event `self.ReceivePossess`
  (params (PossessedPawn :type "Pawn Object Reference"))
  (`self.ResClientProcess`))

(event `ResClientProcess`
  ;[1 1 1] RunOnClientOnly
  (bind _asgmi_animal_guys (cast `/Game/AnimalGuys/1_LeeWoongJae/GameMode/GMI_AnimalGuys` (`GameplayStatics.GetGameInstance`)))
  (`self.ReqUpdatePlayerInfo` (`/Game/AnimalGuys/1_LeeWoongJae/GameMode/GMI_AnimalGuys.DBPlayerInfo` _asgmi_animal_guys) self))

(event `ReqUpdatePlayerInfo`
  (params (PlayerInfo :type "/Game/AnimalGuys/1_LeeWoongJae/Network/ST_PlayerInfo Structure") (PlayerController :type "PlayerController Object Reference"))
  ;[1 1 1] RunOnServer
  (bind _asps_animal_guys_lobby (cast `/Game/AnimalGuys/1_LeeWoongJae/GameMode/PS_AnimalGuys_Lobby` (`self.PlayerState`)))
  (set `/Game/AnimalGuys/1_LeeWoongJae/GameMode/PS_AnimalGuys_Lobby.PlayerControllerRef` PlayerController _asps_animal_guys_lobby)
  (`/Game/AnimalGuys/1_LeeWoongJae/GameMode/PS_AnimalGuys_Lobby.SetPlayerInfo` _asps_animal_guys_lobby PlayerInfo))

(fn `UserConstructionScript`)